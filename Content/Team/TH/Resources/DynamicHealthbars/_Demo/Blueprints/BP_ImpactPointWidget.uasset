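; BP_ImpactPointWidget is a demo Blueprint in DynamicHealthbars that shows a bullet impact marker when enemies are hit.
; It acts as a thin wrapper around a Widget_Hit hosted in its WidgetHit component.
; Initialise stores the actor being hit and passes it to that widget, while the Activate event triggers the widget's own Activate.
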(event `Activate`
  ;[1 1 1] Activate the impact point widget
  (bind _aswidget_hit (cast `/Game/Team/TH/Resources/DynamicHealthbars/_Demo/Blueprints/Widgets/Widget_Hit` (`WidgetComponent.GetUserWidgetObject` (`self.WidgetHit`))))
  (`/Game/Team/TH/Resources/DynamicHealthbars/_Demo/Blueprints/Widgets/Widget_Hit.Activate` _aswidget_hit false))

(fn `Initialise`
  (params (ActorBeingHit :type "Actor Object Reference"))
  ;[1 1 1] Blueprint for showing the impact decal of bullets (when hitting enemies)
  (set `self.ActorBeingHit` ActorBeingHit)
  (bind _aswidget_hit (cast `/Game/Team/TH/Resources/DynamicHealthbars/_Demo/Blueprints/Widgets/Widget_Hit` (`WidgetComponent.GetUserWidgetObject` (`self.WidgetHit`))))
  (set `/Game/Team/TH/Resources/DynamicHealthbars/_Demo/Blueprints/Widgets/Widget_Hit.ActorBeingHit` (`self.ActorBeingHit`) _aswidget_hit))

(fn `UserConstructionScript`)