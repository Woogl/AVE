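; BPC_Swordman is a swordsman enemy Blueprint that sets up an HP and posture display through its EnemyWidget component.
; On BeginPlay it creates a UI_GunEnemyHP widget, stores it as BitalInfo and assigns it to EnemyWidget.
; It passes the maximum HP and posture to the widget, then refreshes it once with the current values.
; The graph holds no combat, overlap or per-tick logic.
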(event `self.ReceiveBeginPlay`
  (bind _bitalinfo (`self.BitalInfo`))
  (bind _returnvalue (`|CreateWidget` "/Game/Team/YEJ/GunEnemy/UI/UI_GunEnemyHP.UI_GunEnemyHP_C"))
  (bind _output_get (set `self.BitalInfo` _returnvalue))
  (`WidgetComponent.SetWidget` (`self.enemyWidget`) _output_get)
  (`/Game/Team/YEJ/GunEnemy/UI/UI_GunEnemyHP.SetInfo` _bitalinfo (`self.hpMax`) (`self.postureMax`))
  (`/Game/Team/YEJ/GunEnemy/UI/UI_GunEnemyHP.Refresh` _bitalinfo (`self.hp`) (`self.posture`)))

(fn `UserConstructionScript`)