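; Third-person shooter player character with mouse look, jump, controller-relative movement and a crosshair widget added on BeginPlay.
; Forward/backward input uses DoOnce gates to trigger mesh animations on starting and stopping.
; Left click plays a montage and sound, line-traces along the camera forward vector, spawns a hit effect and damages only BP_Swordman.
; Held-fire logic is disconnected and SetGun is an empty stub.
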(event `self.ReceiveBeginPlay`
  (bind _returnvalue (`|CreateWidget` "/Game/Team/TH/Blueprints/WBP_Crosshair.WBP_Crosshair_C"))
  (`UserWidget.AddToViewport` _returnvalue 0))

(event `InputAxis|Move Forward / Backward`
  (params (AxisValue :type "Float (single-precision)"))
  (bind _mesh (`self.Mesh`))
  (bind (_returnvalue_x _returnvalue_y) (`KismetMathLibrary.BreakVector` (`KismetMathLibrary.TransformDirection` (`self.GetTransform` (`GameplayStatics.GetPlayerController` 0)) (`KismetMathLibrary.MakeVector` (`self.GetInputAxisValue`) (`self.GetInputAxisValue`)))))
  (`self.AddMovementInput` (`KismetMathLibrary.Normal` (`KismetMathLibrary.MakeVector` _returnvalue_x _returnvalue_y)))
  (if (> (`KismetMathLibrary.Abs` AxisValue) 0.3)
    (`/Engine/EditorBlueprintResources/StandardMacros.DoOnce` false :!label _label
      (:`Completed`
        (`SkeletalMeshComponent.PlayAnimation` _mesh null false)
        (goto _label_2 :!via `Reset`)))
    (else
      (`/Engine/EditorBlueprintResources/StandardMacros.DoOnce` false :!label _label_2
        (:`Completed`
          (`SkeletalMeshComponent.PlayAnimation` _mesh null false)
          (goto _label :!via `Reset`))))))

(event `self.ReceiveTick`
  (params (DeltaSeconds :type "Float (single-precision)")))

(event `Key|LeftMouseButton`
  (params (Key :type "Key Structure"))
  (bind _camera (`self.Camera`))
  (:`Pressed`
    (`self.PlayAnimMontage` "/Game/Team/TH/Blueprints/TPSPlayerMontage.TPSPlayerMontage")
    (`GameplayStatics.PlaySoundAtLocation` "/Engine/VREditor/Sounds/UI/Flashlight_Switch.Flashlight_Switch" (`self.K2_GetActorLocation`) (struct) 1.0 1.0 0.0 null null null null)
    (bind _outhit (`KismetSystemLibrary.LineTraceSingleByProfile` :`Start` (`SceneComponent.K2_GetComponentLocation` _camera) :`End` (* (`SceneComponent.GetForwardVector` _camera) 300000.0) :`ProfileName` "Pawn" :`DrawDebugType` "ForOneFrame"))
    (`GameplayStatics.SpawnEmitterAtLocation` "/Game/MarketplaceAssets/Cruel_Sword_Finisher/Particles/P_Hit.P_Hit" (`.Location` (`GameplayStatics.BreakHitResult` _outhit)))
    (bind _asbp_swordman (cast `/Game/Team/TH/Blueprints/BP_Swordman` (`.HitActor` (`GameplayStatics.BreakHitResult` _outhit))))
    (`GameplayStatics.ApplyDamage` _asbp_swordman 1.0 (`AIBlueprintHelperLibrary.GetAIController` _asbp_swordman) self "/Script/Engine.DamageType"))
  (:`Released`
    (set `self.Open Fire` false)))

(event `InputAxis|Look Up / Down Mouse` :overrideparent false
  (params (AxisValue :type "Float (single-precision)"))
  (`self.AddControllerPitchInput` AxisValue))

(event `InputAxis|Turn Right / Left Mouse` :overrideparent false
  (params (AxisValue :type "Float (single-precision)"))
  (`self.AddControllerYawInput` AxisValue))

(event `InputAction|Jump` :overrideparent false
  (params (Key :type "Key Structure"))
  (:`Pressed`
    (`self.Jump`)))

(fn `Set Gun`
  (params (isSniperGun :type Boolean)))

(fn `UserConstructionScript`)