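; Katana-wielding enemy character with health, posture, guard and a floating healthbar chosen from preset variations.
; Point damage updates HP, posture and bars, alerts AI through Blackboard and BP_Manager, and picks a reaction montage by DamageType.
; A looping timer restores posture after reactions; depleted posture flags the enemy Broken.
; Death notifies the manager, plays a montage, ragdolls the mesh and spawns a dropped katana.
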(event `self.ReceiveBeginPlay`
  (`|ExecutionSequence`
    (:`then_0`
      (bind _returnvalue (`|SpawnActorFromClass` "/Game/Team/TH/Resources/DynamicHealthbars/_Demo/Blueprints/BP_ImpactPointWidget.BP_ImpactPointWidget_C" (`KismetMathLibrary.MakeTransform` (0.0 0.0 0.0)) "Undefined" "OverrideRootScale" null null))
      (bind _output_get (set `self.ImpactPointWidget` _returnvalue))
      (`/Game/Team/TH/Resources/DynamicHealthbars/_Demo/Blueprints/BP_ImpactPointWidget.Initialise` _output_get self)
      (`self.InitialiseHealthbarVariations` (`self.HealthbarVariationIndex`)))
    (:`then_1`
      (`CombatComponent.SetupWeapon` (`self.CombatComp`) (`self.Katana_hand`))
      (bind _returnvalue_2 (`GameplayStatics.GetActorOfClass` "/Game/Team/TH/Blueprints/BP_Manager.BP_Manager_C"))
      (set `self.AIManager` _returnvalue_2)
      (set `self.Blackboard_0` (`AIBlueprintHelperLibrary.GetBlackboard` self)))))

(event `Dead`
  (bind _mesh (`self.Mesh`))
  (`AIController.K2_ClearFocus` (`AIBlueprintHelperLibrary.GetAIController` self))
  (`BlackboardComponent.SetValueAsEnum` (`self.Blackboard_0`) (`self.AIState`) 3)
  (`PrimitiveComponent.SetCollisionEnabled` (`self.CapsuleComponent`) "PhysicsOnly")
  (`/Game/Team/TH/Blueprints/BP_Manager.EnemyDie` (`self.AIManager`) self)
  (`|PlayMontage` _mesh "/Game/Team/TH/Animation/Mon_SwordmanBreak.Mon_SwordmanBreak" 1.0 0.0 "Death0"
    (:`then`
      (`PrimitiveComponent.SetSimulatePhysics` _mesh true)
      (`|SpawnActorFromClass` "/Game/Team/TH/Blueprints/BP_SwordmanKatana.BP_SwordmanKatana_C" (`SceneComponent.GetSocketTransform` (`self.Mesh`) "hand_rSocket" "RTS_World") "Undefined" "OverrideRootScale" null null)
      (`SceneComponent.K2_DetachFromComponent` (`self.Katana_hand`) "KeepRelative" "KeepRelative" "KeepRelative" true)
      (set `self.hp` 1000000000.0)
      (if (<= (`/Game/Team/TH/Resources/DynamicHealthbars/Blueprints/Widgets/Widget_FloatingHealthbar.GetCurrentValue` (`self.GetHealthBarWidget`) "NewEnumerator0") 0.0)
        (`/Game/Team/TH/Resources/DynamicHealthbars/Blueprints/Widgets/Widget_FloatingHealthbar.OnParentActorDead` (`self.GetHealthBarWidget`))
        (if (not (`self.bHidden`))
          (`GameplayStatics.SpawnEmitterAtLocation` "/Game/Team/TH/Resources/DynamicHealthbars/_Demo/FX/EnemyDeath/P_EnemyDeath.P_EnemyDeath" (0.0 0.0 0.0) (struct) (0.65 0.65 0.65)))))))

(event `PostureBreak`
  (`BlackboardComponent.SetValueAsBool` (`self.Blackboard_0`) (`self.Broken`) true)
  (`BlackboardComponent.SetValueAsBool` (`self.Blackboard_0`) (`self.Guard`) false)
  (set `self.Tags` (`|MakeArray` "Broken" :!type "Name")))

(event `self.ReceivePointDamage`
  (params (Damage :type "Float (single-precision)") (DamageType :type "DamageType Object Reference") (HitLocation :type "Vector Structure") (HitNormal :type "Vector Structure") (HitComponent :type "PrimitiveComponent Object Reference") (BoneName :type Name) (ShotFromDirection :type "Vector Structure") (InstigatedBy :type "Controller Object Reference") (DamageCauser :type "Actor Object Reference") (HitInfo :type "HitResult Structure (by ref)"))
  (bind _returnvalue (`GameplayStatics.GetObjectClass` DamageType))
  (bind _mesh (`self.Mesh`))
  (`self.K2_SetActorLocation` (`self.ImpactPointWidget`) HitLocation false true)
  (`/Game/Team/TH/Resources/DynamicHealthbars/_Demo/Blueprints/BP_ImpactPointWidget.Activate` (`self.ImpactPointWidget`))
  (set `self.bUseControllerRotationYaw` false)
  (`self.Hit` Damage Damage)
  (if (== _returnvalue "/Script/AVE.StandardDamageType")
    (`|PlayMontage` _mesh "/Game/Team/TH/Animation/Mon_SwordmanMove.Mon_SwordmanMove" 1.0 0.0 "Hit0" :!label _label
      (:`OnCompleted`
        _)
      (:`OnInterrupted`
        _))
    (elif (== _returnvalue "/Script/AVE.KnockBackDamageType")
      (`|PlayMontage` _mesh "/Game/Team/TH/Animation/Mon_SwordmanMove.Mon_SwordmanMove" 1.0 0.0 "Hit3"
        (:`OnCompleted`
          _)
        (:`OnInterrupted`
          _))
      (elif (== _returnvalue "/Script/AVE.KnockDownDamageType")
        (`|PlayMontage` _mesh "/Game/Team/TH/Animation/Mon_SwordmanBreak.Mon_SwordmanBreak" 1.0 0.0 "SwordDown"
          (:`OnCompleted`
            _)
          (:`OnInterrupted`
            _))
        (elif (== _returnvalue "/Script/AVE.KnockUpDamageType")
          (`|PlayMontage` _mesh "/Game/Team/TH/Animation/Mon_SwordmanBreak.Mon_SwordmanBreak" 1.0 0.0 "SwordAirBorne"
            (:`OnCompleted`
              _)
            (:`OnInterrupted`
              _))
          (else
            (goto _label))))))
  (set `self.bUseControllerRotationYaw` true)
  (bind _returnvalue_2 (`KismetSystemLibrary.K2_SetTimerDelegate` (delegate `PostureRegen`) 2.0 true 2.0)))

(event `PostureRegen`
  (bind _posture (`self.posture`))
  (if (<= _posture (`self.postureMax`))
    (set `self.posture` (+ _posture 20.0))
    (if (> (`self.posture`) 0.0)
      (set `self.Tags` (`|MakeArray` "None" :!type "Name")))
    (else
      (`KismetSystemLibrary.K2_ClearAndInvalidateTimerHandle` (stale `self.ReceivePointDamage` _returnvalue_2)))))

(fn `GetHealthBarWidget`
  (returns (Widget :type "/Game/Team/TH/Resources/DynamicHealthbars/Blueprints/Widgets/Widget_FloatingHealthbar Object Reference"))
  ;[1 1 1] Helper function to retrieve the healthbar widget
  (bind _aswidget_floating_healthbar (cast `/Game/Team/TH/Resources/DynamicHealthbars/Blueprints/Widgets/Widget_FloatingHealthbar` (`WidgetComponent.GetUserWidgetObject` (`self.FloatingHealthbar`))))
  (return _aswidget_floating_healthbar))

(fn `Hatto`
  (`SceneComponent.SetVisibility` (`self.Katana_hand`) true false)
  (`SceneComponent.SetVisibility` (`self.Katana_waist`) false false))

(fn `Hit`
  (params (Damage :type "Float (double-precision)") (Posture :type "Float (double-precision)"))
  (bind _widget (`self.GetHealthBarWidget`))
  (`/Game/Team/TH/Resources/DynamicHealthbars/Blueprints/Widgets/Widget_FloatingHealthbar.SubtractValue` _widget "NewEnumerator0" Damage)
  (`/Game/Team/TH/Resources/DynamicHealthbars/Blueprints/Widgets/Widget_FloatingHealthbar.SubtractValue` _widget "NewEnumerator1" Posture)
  (`self.Hatto`)
  (`BlackboardComponent.SetValueAsEnum` (`self.Blackboard_0`) (`self.AIState`) 4)
  (`AISense_Damage.ReportDamageEvent` self null 0.0 (`self.K2_GetActorLocation`))
  (`/Game/Team/TH/Blueprints/BP_Manager.Start AI` (`self.AIManager`))
  (if (not (`BlackboardComponent.GetValueAsBool` (`self.Blackboard_0`) (`self.Guard`)))
    (bind _output_get (set `self.hp` (- (`self.hp`) Damage))))
  (bind _output_get_2 (set `self.posture` (`KismetMathLibrary.FClamp` (- (`self.posture`) Posture) 0.0 (`self.postureMax`))))
  (if (<= _output_get 0.0)
    (`self.Dead`)
    (return)
    (elif (<= _output_get_2 0.0)
      (`self.PostureBreak`)
      (return)
      (else
        (return)))))

(fn `InitialiseHealthbarVariations`
  (params (VariationIndex :type Integer))
  (locals (WidgetScale :type "Float (double-precision)" :default 1.2))
  ;[1 1 1] Preset healthbar settings, used by enemies to show variations in the demo level
  (switch `int` VariationIndex
    (:`Default`
      (`/Game/Team/TH/Resources/DynamicHealthbars/Blueprints/Widgets/Widget_FloatingHealthbar.Initialise` :`self` (`self.GetHealthBarWidget`) :`Parent` self :`WidgetScale` (`local.WidgetScale`) :`MaxValue` (`self.hpMax`) :`CanBeOccluded` true :`Material` "/Game/Team/TH/Resources/DynamicHealthbars/Materials/M_Healthbar.M_Healthbar" :`Colour` (struct :`R` 0.546875 :`G` 0.010878 :`A` 1.0) :`NumSegments` 7 :`EliteFrame` true :`DistanceVisible` -1.0 :`OptionalName` "" :`OptionalMultiplayerSettings` (make `/Game/Team/TH/Resources/DynamicHealthbars/Blueprints/Widgets/STRUCT_OtherTeamInfo` null true (struct :`R` 0.042561 :`G` 0.96875 :`B` 0.794164 :`A` 1.0) true "Ally") :!label _label))
    (:`0`
      (goto _label))
    (:`1`
      (goto _label))
    (:`2`
      (`/Game/Team/TH/Resources/DynamicHealthbars/Blueprints/Widgets/Widget_FloatingHealthbar.Initialise` :`self` (`self.GetHealthBarWidget`) :`Parent` self :`WidgetScale` (`local.WidgetScale`) :`MaxValue` (`self.hpMax`) :`Level` 7 :`CanBeOccluded` true :`Material` "/Game/Team/TH/Resources/DynamicHealthbars/Materials/M_Healthbar.M_Healthbar" :`Colour` (struct :`R` 0.432361 :`G` 0.086717 :`B` 0.546875 :`A` 1.0) :`DistanceVisible` -1.0 :`OptionalName` "Enemy Name"))
    (:`3`
      (`/Game/Team/TH/Resources/DynamicHealthbars/Blueprints/Widgets/Widget_FloatingHealthbar.Initialise` :`self` (`self.GetHealthBarWidget`) :`Parent` self :`WidgetScale` (`local.WidgetScale`) :`MaxValue` (`self.hpMax`) :`CanBeOccluded` true :`Material` "/Game/Team/TH/Resources/DynamicHealthbars/Materials/M_HealthBar_Pattern2_Mat.M_HealthBar_Pattern2_Mat" :`Colour` (struct :`R` 0.546875 :`G` 0.546875 :`B` 0.546875 :`A` 1.0) :`ShowPercentage` true :`DistanceVisible` -1.0 :`OptionalName` "Animated Bar" :`OptionalNameSettings` (make `/Game/Team/TH/Resources/DynamicHealthbars/Blueprints/Widgets/STRUCT_OptionalNameSettings` 13 (struct :`R` 0.204164 :`G` 1.0 :`B` 0.297275 :`A` 1.0))))
    (:`4`
      (`/Game/Team/TH/Resources/DynamicHealthbars/Blueprints/Widgets/Widget_FloatingHealthbar.Initialise` :`self` (`self.GetHealthBarWidget`) :`Parent` self :`WidgetScale` (`local.WidgetScale`) :`MaxValue` (`self.hpMax`) :`CanBeOccluded` true :`Material` "/Game/Team/TH/Resources/DynamicHealthbars/Materials/M_HealthBar_Pattern3_Mat.M_HealthBar_Pattern3_Mat" :`Colour` (struct :`R` 0.546875 :`G` 0.546875 :`B` 0.546875 :`A` 1.0) :`ShowPercentage` true :`DistanceVisible` -1.0 :`OptionalName` "Status Effects"))
    (:`5`
      (`/Game/Team/TH/Resources/DynamicHealthbars/Blueprints/Widgets/Widget_FloatingHealthbar.Initialise` :`self` (`self.GetHealthBarWidget`) :`Parent` self :`WidgetScale` (`local.WidgetScale`) :`MaxValue` (`self.hpMax`) :`Level` 27 :`CanBeOccluded` true :`Material` "/Game/Team/TH/Resources/DynamicHealthbars/Materials/M_Healthbar.M_Healthbar" :`EliteFrame` true :`ShowPercentage` true :`DistanceVisible` -1.0 :`OptionalName` "Elite Frame" :`OptionalNameSettings` (make `/Game/Team/TH/Resources/DynamicHealthbars/Blueprints/Widgets/STRUCT_OptionalNameSettings` 13 (struct :`R` 0.651604 :`G` 0.65625 :`B` 0.222168 :`A` 1.0))))
    (:`6`
      (`/Game/Team/TH/Resources/DynamicHealthbars/Blueprints/Widgets/Widget_FloatingHealthbar.Initialise` :`self` (`self.GetHealthBarWidget`) :`Parent` self :`WidgetScale` (`local.WidgetScale`) :`MaxValue` (`self.hpMax`) :`Level` 15 :`CanBeOccluded` true :`Material` "/Game/Team/TH/Resources/DynamicHealthbars/Materials/M_HealthBar_Pattern_Mat.M_HealthBar_Pattern_Mat" :`Colour` (struct :`R` 0.546875 :`G` 0.546875 :`B` 0.546875 :`A` 1.0) :`Shear` -12.0 :`ShowPercentage` true :`DistanceVisible` -1.0 :`OptionalName` "Foot Soldier"))
    (:`7`
      (`/Game/Team/TH/Resources/DynamicHealthbars/Blueprints/Widgets/Widget_FloatingHealthbar.Initialise` :`self` (`self.GetHealthBarWidget`) :`Parent` self :`WidgetScale` (`local.WidgetScale`) :`MaxValue` (`self.hpMax`) :`Level` 15 :`CanBeOccluded` true :`Material` "/Game/Team/TH/Resources/DynamicHealthbars/Materials/M_Healthbar.M_Healthbar" :`Colour` (struct :`R` 0.546875 :`G` 0.48394 :`B` 0.063736 :`A` 1.0) :`Shear` -15.0 :`DistanceVisible` -1.0 :`OptionalName` "Assassin"))
    (:`8`
      (`/Game/Team/TH/Resources/DynamicHealthbars/Blueprints/Widgets/Widget_FloatingHealthbar.Initialise` :`self` (`self.GetHealthBarWidget`) :`Parent` self :`WidgetScale` (`local.WidgetScale`) :`MaxValue` (`self.hpMax`) :`CanBeOccluded` true :`Material` "/Game/Team/TH/Resources/DynamicHealthbars/Materials/M_HealthBar_Pattern3_Mat.M_HealthBar_Pattern3_Mat" :`Colour` (struct :`R` 0.546875 :`G` 0.546875 :`B` 0.546875 :`A` 1.0) :`DistanceVisible` -1.0 :`OptionalName` "Large Name" :`OptionalNameSettings` (make `/Game/Team/TH/Resources/DynamicHealthbars/Blueprints/Widgets/STRUCT_OptionalNameSettings` 21)))
    (:`9`
      (`/Game/Team/TH/Resources/DynamicHealthbars/Blueprints/Widgets/Widget_FloatingHealthbar.Initialise` :`self` (`self.GetHealthBarWidget`) :`Parent` self :`WidgetScale` (`local.WidgetScale`) :`MaxValue` (`self.hpMax`) :`CanBeOccluded` true :`HideIfMainBarFull` true :`Material` "/Game/Team/TH/Resources/DynamicHealthbars/Materials/M_Healthbar.M_Healthbar" :`Colour` (struct :`R` 0.546875 :`G` 0.010878 :`A` 1.0) :`Shear` -12.0 :`DistanceVisible` -1.0 :`OptionalName` "" :`OptionalBar1` (make `/Game/Team/TH/Resources/DynamicHealthbars/Blueprints/Widgets/STRUCT_BarInfo` (`self.postureMax`) (struct :`R` 0.111076 :`G` 0.338542 :`B` 0.09247 :`A` 1.0))))
    (:`10`
      (`/Game/Team/TH/Resources/DynamicHealthbars/Blueprints/Widgets/Widget_FloatingHealthbar.Initialise` :`self` (`self.GetHealthBarWidget`) :`Parent` self :`WidgetScale` (`local.WidgetScale`) :`MaxValue` (`self.hpMax`) :`Level` 15 :`CanBeOccluded` true :`Material` "/Game/Team/TH/Resources/DynamicHealthbars/Materials/M_Healthbar.M_Healthbar" :`Colour` (struct :`R` 0.546875 :`G` 0.010878 :`A` 1.0) :`EliteFrame` true :`ShowPercentage` true :`DistanceVisible` -1.0 :`OptionalName` "More Bars" :`OptionalBar1` (make `/Game/Team/TH/Resources/DynamicHealthbars/Blueprints/Widgets/STRUCT_BarInfo` 100.0 (struct :`R` 0.75 :`G` 0.695466 :`B` 0.065169 :`A` 1.0)) :`OptionalBar2` (make `/Game/Team/TH/Resources/DynamicHealthbars/Blueprints/Widgets/STRUCT_BarInfo` 100.0 (struct :`G` 0.371795 :`B` 0.75 :`A` 1.0)) :`OptionalBar3` (make `/Game/Team/TH/Resources/DynamicHealthbars/Blueprints/Widgets/STRUCT_BarInfo` 100.0 (struct :`R` 0.75 :`G` 0.077943 :`B` 0.475999 :`A` 1.0))))))

(fn `UserConstructionScript`)