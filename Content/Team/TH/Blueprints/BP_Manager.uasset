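; BP_Manager is an AI-driven manager that runs BT_Manager and coordinates a list of enemies against the player.
; When TurnedOn, StartAI clears the flag, stores the player in its blackboard, calls OnGetSet on each enemy and writes their AIState.
; The AIState exclusion check joins inequalities with OR, so it always passes.
; TurnedOn re-arms through FastAttack's random roll or when EnemyDie empties the list.
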(event `self.ReceiveBeginPlay`
  (set `self.PlayerActor` (`GameplayStatics.GetPlayerPawn` 0))
  (`AIController.RunBehaviorTree` (`AIBlueprintHelperLibrary.GetAIController` self) "/Game/Team/TH/Tree/Manager/BT_Manager.BT_Manager"))

(fn `EnemyDie`
  (params (EnemyActor :type "/Game/Team/TH/Blueprints/BP_Swordman Object Reference"))
  (bind _enemies (`self.Enemies`))
  (`KismetArrayLibrary.Array_RemoveItem` _enemies EnemyActor)
  (if (`KismetArrayLibrary.Array_IsEmpty` _enemies)
    (set `self.TurnedOn` true)))

(fn `FastAttack`
  (if (>= (`KismetMathLibrary.RandomIntegerInRange` 0 9) (`self.AttackChance`))
    (set `self.TurnedOn` true)))

(fn `Start AI`
  (locals (AIState :type Name :default "AIState") (Enum :type Byte :default 1) (Player :type Name :default "PlayerActor"))
  (if (`self.TurnedOn`)
    (set `self.TurnedOn` false)
    (`BlackboardComponent.SetValueAsObject` (`AIBlueprintHelperLibrary.GetBlackboard` null) (`local.Player`) (`self.PlayerActor`))
    (for _array_element (`self.Enemies`)
      (bind _asenemy_base (cast `EnemyBase` _array_element))
      (`EnemyBase.onGetSet` _asenemy_base)
      (bind _returnvalue (`AIBlueprintHelperLibrary.GetBlackboard` _asenemy_base))
      (bind _returnvalue_2 (`BlackboardComponent.GetValueAsEnum` _returnvalue (`local.AIState`)))
      (if (or (!= _returnvalue_2 3) (!= _returnvalue_2 4) (!= _returnvalue_2 5))
        (`BlackboardComponent.SetValueAsEnum` _returnvalue (`local.AIState`) (`local.Enum`))))))

(fn `UserConstructionScript`)