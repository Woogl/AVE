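; BP_SpearEnemy is a halberd-wielding melee enemy with a world-space health and posture bar turned toward the player each tick.
; SpearAttack, meant for a Behavior Tree task, faces the player, plays one of three random montages and applies damage immediately, while weapon overlap adds fixed damage.
; Incoming damage updates the bar and plays a hit montage; the ragdoll Die branch tests HP below zero after clamping to zero, so never triggers.
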(event `SpearAttack`
  (bind _returnvalue (`GameplayStatics.GetPlayerPawn` 0))
  ;[0 0 0] 플레이어 공격(BT Task와 연결)
  (`self.K2_SetActorRotation` (`KismetMathLibrary.FindLookAtRotation` (`self.K2_GetActorLocation`) (`self.K2_GetActorLocation` (`GameplayStatics.GetPlayerCharacter` 0))))
  (bind _output_get (set `self.AttackCombo` (`KismetMathLibrary.RandomIntegerInRange` 0 2)))
  (switch `int` _output_get
    (:`0`
      (`GameplayStatics.ApplyDamage` _returnvalue (`self.Attack1Damage`) null self "/Script/AVE.StandardDamageType")
      (`self.PlayAnimMontage` "/Game/Team/YEJ/SpearEnemy/Animation/Montage/ARPG_Halberd_Anim_UE_Attack_Combo1_Montage.ARPG_Halberd_Anim_UE_Attack_Combo1_Montage"))
    (:`1`
      (`GameplayStatics.ApplyDamage` _returnvalue (`self.Attack2Damage`) null self "/Script/AVE.StandardDamageType")
      (`self.PlayAnimMontage` "/Game/Team/YEJ/SpearEnemy/Animation/Montage/ARPG_Halberd_Anim_UE_Attack_Combo4_Montage.ARPG_Halberd_Anim_UE_Attack_Combo4_Montage"))
    (:`2`
      (`GameplayStatics.ApplyDamage` _returnvalue (`self.Attack3Damage`) null self "/Script/AVE.StandardDamageType")
      (`self.PlayAnimMontage` "/Game/Team/YEJ/SpearEnemy/Animation/Montage/ARPG_Halberd_Anim_UE_Attack_Heavy2_Montage.ARPG_Halberd_Anim_UE_Attack_Heavy2_Montage"))))

(event `self.ReceiveTick`
  (params (DeltaSeconds :type "Float (single-precision)"))
  (bind _widget (`self.Widget`))
  ;[0 0 0] 월드상 어디에서든 위젯바가 제대로 보이게
  (`SceneComponent.K2_SetWorldRotation` _widget (`KismetMathLibrary.FindLookAtRotation` (`SceneComponent.K2_GetComponentLocation` _widget) (`self.K2_GetActorLocation` (`GameplayStatics.GetPlayerCharacter` 0))) false false))

(event `self.ReceiveBeginPlay`
  (bind _target (`self.Target`))
  ;[0 0 0] SpearEnemy HP 설정
  (set `self.CurrentHP` (`self.Max HP`))
  (bind _returnvalue (`|CreateWidget` "/Game/Team/YEJ/SpearEnemy/Blueprint/UI_SpearEnemyHP.UI_SpearEnemyHP_C"))
  (bind _output_get (set `self.SpearUI` _returnvalue))
  (`WidgetComponent.SetWidget` (`self.Widget`) _output_get)
  (`/Game/Team/YEJ/GunEnemy/UI/UI_GunEnemyHP.SetInfo` _target (`self.Max HP`) (`self.Max Posture`))
  (`/Game/Team/YEJ/GunEnemy/UI/UI_GunEnemyHP.Refresh` _target (`self.CurrentHP`) (`self.Now Posture`)))

(event `self.WeaponCollision.OnComponentBeginOverlap`
  (params (OverlappedComponent :type "PrimitiveComponent Object Reference") (OtherActor :type "Actor Object Reference") (OtherComp :type "PrimitiveComponent Object Reference") (OtherBodyIndex :type Integer) (bFromSweep :type Boolean) (SweepResult :type "HitResult Structure (by ref)"))
  ;[0 0 0] 데미지 입히기(플레이어 피격 이벤트 필요)
  (bind _asbp_new_player_character (cast `/Game/Blueprints/BP_NewPlayerCharacter` OtherActor))
  (`GameplayStatics.ApplyDamage` _asbp_new_player_character 10.0 null self "/Script/AVE.StandardDamageType"))

(event `self.ReceiveAnyDamage`
  (params (Damage :type "Float (single-precision)") (DamageType :type "DamageType Object Reference") (InstigatedBy :type "Controller Object Reference") (DamageCauser :type "Actor Object Reference"))
  ;[0 0 0] 데미지 받음(피격)
  (bind _output_get (set `self.CurrentHP` (`KismetMathLibrary.FClamp` (- (`self.CurrentHP`) Damage) 0.0 (`self.Max HP`))))
  (`/Game/Team/YEJ/GunEnemy/UI/UI_GunEnemyHP.Refresh` (`self.Target`) (`self.CurrentHP`) (`self.Now Posture`))
  ;[0 0 0] HP 구분/ 사느냐 죽느냐
  (if (< _output_get 0.0)
    (set `self.IsAlive` false)
    (`self.Die`)
    (else
      (set `self.IsAlive` true)
      (`self.PlayAnimMontage` "/Game/Team/YEJ/SpearEnemy/Animation/Montage/ARPG_Halberd_Anim_UE_Executed2_Montage.ARPG_Halberd_Anim_UE_Executed2_Montage"))))

(event `Die`
  ;[0 0 0] HP가 0이 되면 사망
  (`/Engine/EditorBlueprintResources/StandardMacros.DoOnce` false
    (:`Completed`
      (`self.PlayAnimMontage` "/Game/Team/YEJ/SpearEnemy/Animation/Montage/ARPG_Halberd_Anim_UE_Death2_Montage.ARPG_Halberd_Anim_UE_Death2_Montage")
      (`PrimitiveComponent.SetSimulatePhysics` (`self.Mesh`) true)
      (`self.DisableInput` (`GameplayStatics.GetPlayerController` 0))
      (`SceneComponent.K2_DetachFromComponent` (`self.Widget`) "KeepRelative" "KeepRelative" "KeepRelative" true))))

(fn `UserConstructionScript`)