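; AC_Boss is an AI controller Blueprint for the boss, with its possess, begin play and tick events left empty.
; Disconnected nodes sketch behavior tree and blackboard startup, a BP_Boss cast, and updates of the player target and distance keys, but none of them run.
; SetFocusToPlayer sets its own actor's yaw toward the stored third-person character, though nothing in this file calls it or assigns that character.
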(event `self.ReceivePossess`
  (params (PossessedPawn :type "Pawn Object Reference")))

(event `self.ReceiveBeginPlay`)

(event `self.ReceiveTick`
  (params (DeltaSeconds :type "Float (single-precision)")))

(fn `SetFocusToPlayer`
  (bind (_returnvalue_roll _returnvalue_pitch _returnvalue_yaw) (`KismetMathLibrary.BreakRotator` (`KismetMathLibrary.FindLookAtRotation` (`self.K2_GetActorLocation`) (`self.K2_GetActorLocation` (`self.As BP Third Person Character`)))))
  (`self.K2_SetActorRotation` (`KismetMathLibrary.MakeRotator` 0.0 0.0 _returnvalue_yaw)))

(fn `UserConstructionScript`)