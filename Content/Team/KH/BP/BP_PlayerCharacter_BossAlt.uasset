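; Player character Blueprint that implements combat presentation events, some declared in C++, for skills, finishers and effects.
; Motion warp events place the player at set distances from EnemyTarget, facing it, for Ganpa and grab-hit moves.
; Skill events share CameraMove, which blends to a sequence camera, plays the sequence, then restores the follow camera by timer.
; It also spawns ghost trails, creates stat and screen-cut widgets, and notifies finished Dummy targets.
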(event `self.MotionMorph`)

(event `self.MotionMorphGanpa`
  (bind (_returnvalue_roll _returnvalue_pitch) (`KismetMathLibrary.BreakRotator` (`self.K2_GetActorRotation`)))
  (bind _returnvalue (`self.K2_GetActorLocation` (`self.EnemyTarget`)))
  (bind (_returnvalue_roll_2 _returnvalue_pitch_2 _returnvalue_yaw) (`KismetMathLibrary.BreakRotator` (`KismetMathLibrary.FindLookAtRotation` (`self.K2_GetActorLocation`) (`self.K2_GetActorLocation` (`self.EnemyTarget`)))))
  (`MotionWarpingComponent.AddOrUpdateWarpTargetFromLocationAndRotation` (`self.MotionWarping`) "Ganpa" (+ (* (`KismetMathLibrary.Normal` (- (`self.K2_GetActorLocation`) _returnvalue)) 500.0) _returnvalue) (`KismetMathLibrary.MakeRotator` _returnvalue_roll _returnvalue_pitch _returnvalue_yaw)))

(event `self.SpawnGhostTrail`
  ;[1 1 1] 잔상
  (`|SpawnActorFromClass` "/Game/Team/Woogle/BP_GhostTrail.BP_GhostTrail_C" (`SceneComponent.K2_GetComponentToWorld` (`self.Mesh`)) "AlwaysSpawn" "OverrideRootScale" null self null))

(event `/Game/Blueprints/BPI_Player.SetRInterpSpeed`
  (params (RInterpSpeed :type "Float (double-precision)"))
  ;[1 1 1] Anim Notify
  (set `self.RInterpSpeed` RInterpSpeed))

(event `self.MotionMorphGrabHit`
  (bind (_returnvalue_roll _returnvalue_pitch) (`KismetMathLibrary.BreakRotator` (`self.K2_GetActorRotation`)))
  (bind _returnvalue (`self.K2_GetActorLocation` (`self.EnemyTarget`)))
  (bind (_returnvalue_roll_2 _returnvalue_pitch_2 _returnvalue_yaw) (`KismetMathLibrary.BreakRotator` (`KismetMathLibrary.FindLookAtRotation` (`self.K2_GetActorLocation`) (`self.K2_GetActorLocation` (`self.EnemyTarget`)))))
  (`MotionWarpingComponent.AddOrUpdateWarpTargetFromLocationAndRotation` (`self.MotionWarping`) "GrabHit" (+ (* (`KismetMathLibrary.Normal` (- (`self.K2_GetActorLocation`) _returnvalue)) 100.0) _returnvalue) (`KismetMathLibrary.MakeRotator` _returnvalue_roll _returnvalue_pitch _returnvalue_yaw)))

(event `self.ReceiveBeginPlay`
  ;[1 1 1] 체력/체간 위젯(임시), 0번 스킬 반갈죽 이펙트용 위젯
  (bind _returnvalue (`|CreateWidget` "/Game/Team/Mun/WBP_PlayerStat.WBP_PlayerStat_C"))
  (bind _output_get (set `self.Widget_PlayerStat` _returnvalue))
  (`UserWidget.AddToViewport` _output_get 0)
  (bind _returnvalue_2 (`|CreateWidget` "/Game/Team/Mun/JudgementCut/WBP_ScreenCut.WBP_ScreenCut_C"))
  (set `self.Widget_ScreenCut` _returnvalue_2))

(event `self.PlayFinisherSequence`
  ;[1 1 1] 스킬 시퀀스
  (`self.CameraMove` (`self.Sequence_Finisher`)))

(event `self.PlayLightningShockSequence`
  ;[1 1 1] 스킬 시퀀스
  (`self.CameraMove` (`self.Sequence_Lightning`)))

(event `self.PlayJudgementCutSequence`
  ;[1 1 1] 스킬 시퀀스
  (`self.CameraMove` (`self.Sequence_JudgementCut`)))

(event `self.PlayMissileSequence`
  ;[1 1 1] 스킬 시퀀스
  (`self.CameraMove` (`self.Sequence_Missile`)))

(event `InputAction|AttackTest`
  (params (Key :type "Key Structure")))

(event `self.PlayEarthquakeSequence`
  ;[1 1 1] 스킬 시퀀스
  (`self.CameraMove` (`self.Sequence_Earthquake`)))

(fn `CameraMove`
  (params (Sequence :type "ActorSequenceComponent Object Reference"))
  (bind _sequenceplayer (`ActorSequenceComponent.SequencePlayer` Sequence))
  (bind _returnvalue (`TimeManagementBlueprintLibrary.Conv_QualifiedFrameTimeToSeconds` (`MovieSceneSequencePlayer.GetDuration` _sequenceplayer)))
  (`PlayerController.SetViewTargetWithBlend` (`GameplayStatics.GetPlayerController` 0) (`ChildActorComponent.ChildActor` (`self.SequenceCameraTarget`)) 0.2 "VTBlend_EaseInOut" 1.0 false)
  (`MovieSceneSequencePlayer.Play` _sequenceplayer)
  (`KismetSystemLibrary.PrintString` (`KismetStringLibrary.Conv_DoubleToString` _returnvalue))
  (`KismetSystemLibrary.K2_SetTimer` null "EndSequence" _returnvalue))

(fn `EndSequence`
  (`PlayerController.SetViewTargetWithBlend` (`GameplayStatics.GetPlayerController` 0) (`ChildActorComponent.ChildActor` (`self.FollowCameraTarget`)) 0.2 "VTBlend_EaseInOut" 1.0 false))

(fn `ScreenCut`
  (bind _widget_screencut (`self.Widget_ScreenCut`))
  (`/Game/Team/Mun/JudgementCut/WBP_ScreenCut.Init` _widget_screencut)
  (`UserWidget.AddToViewport` _widget_screencut 0))

(fn `UserConstructionScript`)