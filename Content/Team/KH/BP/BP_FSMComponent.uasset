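; Boss AI component: a Tick-driven state machine moving BP_Boss through idle, walking, chasing, attacks, backstep and guard.
; A clamped per-state counter, reset on most transitions, separates first-tick setup from later attack triggers and repeated movement updates.
; Player distance, facing yaw and random rolls choose attacks, and a player attack can trigger Guard.
; Boss animation calls return delays that time follow-up moves and returns to MoveTo or Walk.
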(event `SetWalkRandomInt`
  (set `self.WalkRandomInt` (`KismetMathLibrary.RandomIntegerInRange` 1 2))
  (bind _returnvalue (`KismetSystemLibrary.K2_SetTimerDelegate` (delegate `SelectRandomInt`) 5.0 true))
  (set `self.WRI_TimerHandle` _returnvalue))

(event `SelectRandomInt`
  (set `self.WalkRandomInt` (`KismetMathLibrary.RandomIntegerInRange` 1 2)))

(event `self.ReceiveBeginPlay`
  (bind _returnvalue (`self.GetOwner`))
  (set `self.As Owner` _returnvalue)
  (bind _asbp_boss (cast `/Game/Team/KH/BP/BP_Boss` _returnvalue))
  (set `self.As BP Boss` _asbp_boss)
  (bind _asabp_boss (cast `/Game/Team/KH/Anim/ABP_Boss` (`SkeletalMeshComponent.GetAnimInstance` (`Character.Mesh` (`self.As BP Boss`)))))
  (set `self.As ABP Boss` _asabp_boss)
  (set `self.BossStates` "NewEnumerator5"))

(event `IdleFSM`
  (bind _output_get (set `self.IdleRandomDelay` (`KismetMathLibrary.RandomFloatInRange` 0.5 1.5)))
  (`KismetSystemLibrary.Delay` _output_get)
  (`self.SetWalkRandomInt`)
  (set `self.BossStates` "NewEnumerator2")
  (set `self.SequenceValue` 0))

(event `WalkFSM`
  (bind _output_get (set `self.WalkRandomDelay` (`KismetMathLibrary.RandomFloatInRange` 2.0 4.0)))
  (`KismetSystemLibrary.Delay` _output_get)
  (if (> (`KismetMathLibrary.Abs` (`/Game/Team/KH/BP/BP_Boss.Yaw` (`self.As BP Boss`))) 120.0)
    (set `self.BossStates` "NewEnumerator12")
    (set `self.SequenceValue` 0)
    (else
      (set `self.BossStates` "NewEnumerator0")
      (set `self.SequenceValue` 0)))
  (`KismetSystemLibrary.K2_ClearAndInvalidateTimerHandle` (`self.WRI_TimerHandle`)))

(event `MoveToFSM`
  (bind _distancebosstoplayer (`/Game/Team/KH/BP/BP_Boss.DistanceBossToPlayer` (`self.As BP Boss`)))
  (if (and (<= (`self.RandomPercentage`) (`self.DashAttackPercentage`)) (<= _distancebosstoplayer 700.0) (> _distancebosstoplayer 600.0))
    (set `self.BossStates` "NewEnumerator7")
    (set `self.SequenceValue` 0)
    (elif (<= _distancebosstoplayer 250.0)
      (if (> (`KismetMathLibrary.Abs` (`/Game/Team/KH/BP/BP_Boss.Yaw` (`self.As BP Boss`))) 120.0)
        (set `self.BossStates` "NewEnumerator12")
        (set `self.SequenceValue` 0)
        (else
          (set `self.BossStates` "NewEnumerator3")
          (set `self.SequenceValue` 0)))
      (else
        (set `self.BossStates` "NewEnumerator0")
        (set `self.SequenceValue` 0)))))

(event `self.ReceiveTick`
  (params (DeltaSeconds :type "Float (single-precision)"))
  (bind _as_bp_boss (`self.As BP Boss`))
  (bind _as_bp_boss_2 (`self.As BP Boss`))
  (switch `/Game/Team/KH/BP/E_BossFSM_BP` (`self.BossStates`)
    (:`NewEnumerator5`
      ;[1 1 1] Idle
      (bind _returnvalue (`self.IncreaseToMaxInt` 1 2))
      (switch `int` _returnvalue
        (:`1`
          (`self.IdleFSM`))
        (:`2`
          (`self.SetZeroSpeed`)
          (message `/Game/Team/KH/BP/BPI_Boss.SetFocusPlayer` (`self.As Owner`)))))
    (:`NewEnumerator2`
      ;[1 1 1] Walk
      (bind _returnvalue_2 (`self.IncreaseToMaxInt` 1 2))
      (switch `int` _returnvalue_2
        (:`1`
          (`self.WalkFSM`))
        (:`2`
          (`self.SetWalkSpeed`)
          (`/Game/Team/KH/BP/BP_Boss.WalkToLocation` (`self.As BP Boss`))
          (message `/Game/Team/KH/BP/BPI_Boss.SetFocusPlayer` (`self.As Owner`)))))
    (:`NewEnumerator0`
      ;[1 1 1] Move To
      (bind _returnvalue_3 (`self.IncreaseToMaxInt` 1 2))
      (switch `int` _returnvalue_3
        (:`1`
          (set `self.RandomPercentage` (`KismetMathLibrary.RandomFloatInRange` 0.0 1.0)))
        (:`2`
          (`self.SetRunSpeed`)
          (`/Game/Team/KH/BP/BP_Boss.MoveTo` (`self.As BP Boss`))
          (`self.MoveToFSM`)
          (message `/Game/Team/KH/BP/BPI_Boss.SetFocusPlayer` (`self.As Owner`)))))
    (:`NewEnumerator7`
      ;[1 1 1] Dash Attack
      (bind _returnvalue_4 (`self.IncreaseToMaxInt` 1 3))
      (switch `int` _returnvalue_4
        (:`1`
          (`self.RandomInt` 1 2))
        (:`2`
          (if (not (`AnimInstance.IsAnyMontagePlaying` (`self.As ABP Boss`)))
            (switch `int` (`self.AttackRandomInt`)
              (:`1`
                (bind _returnvalue_5 (`/Game/Team/KH/BP/BP_Boss.AnimDashAttack` (`self.As BP Boss`)))
                (`KismetSystemLibrary.Delay` _returnvalue_5)
                (`self.ReturnToMoveTo`))
              (:`2`
                (`self.GoToATK01`)))))
        (:`3`
          (`self.SetZeroSpeed`))))
    (:`NewEnumerator3`
      ;[1 1 1] Normal Attack
      (bind _returnvalue_6 (`self.IncreaseToMaxInt` 1 3))
      (switch `int` _returnvalue_6
        (:`1`
          (`self.RandomInt` 1 2))
        (:`2`
          (if (not (`AnimInstance.IsAnyMontagePlaying` (`self.As ABP Boss`)))
            (bind _returnvalue_7 (`/Game/Team/KH/BP/BP_Boss.Anim Normal Attack` (`self.As BP Boss`)))
            (`KismetSystemLibrary.Delay` _returnvalue_7)
            (`self.ReturnToMoveTo`)))
        (:`3`
          (`self.SetZeroSpeed`)
          (message `/Game/Team/KH/BP/BPI_Boss.SetFocusPlayer` (`self.As Owner`))
          (`self.GoToGuard`))))
    (:`NewEnumerator9`
      ;[1 1 1] ATK01
      (bind _returnvalue_8 (`self.IncreaseToMaxInt` 1 2))
      (switch `int` _returnvalue_8
        (:`1`
          (if (not (`AnimInstance.IsAnyMontagePlaying` (`self.As ABP Boss`)))
            (bind _returnvalue_9 (`/Game/Team/KH/BP/BP_Boss.AnimATK01` (`self.As BP Boss`)))
            (`KismetSystemLibrary.Delay` _returnvalue_9)
            (`self.ReturnToMoveTo`)))
        (:`2`
          (`self.SetZeroSpeed`)
          (`/Game/Team/KH/BP/BP_Boss.SetFocusPlayerSpeed` (`self.As BP Boss`) 0.3))))
    (:`NewEnumerator6`
      ;[1 1 1] Jump Attack
      (bind _returnvalue_10 (`self.IncreaseToMaxInt` 1 3))
      (switch `int` _returnvalue_10
        (:`1`
          (`self.RandomInt` 1 2))
        (:`2`
          (if (not (`AnimInstance.IsAnyMontagePlaying` (`self.As ABP Boss`)))
            (bind _returnvalue_11 (`/Game/Team/KH/BP/BP_Boss.AnimJumpAttack` (`self.As BP Boss`)))
            (`KismetSystemLibrary.Delay` _returnvalue_11)
            (switch `int` (`self.AttackRandomInt`)
              (:`1`
                (bind _returnvalue_12 (`/Game/Team/KH/BP/BP_Boss.AnimStanceToLow` _as_bp_boss_2))
                (`KismetSystemLibrary.Delay` _returnvalue_12)
                (`self.ReturnToMoveTo`))
              (:`2`
                (bind _returnvalue_13 (`/Game/Team/KH/BP/BP_Boss.AnimStanceToStab` _as_bp_boss_2))
                (`KismetSystemLibrary.Delay` _returnvalue_13)
                (`self.ReturnToWalk`)))))
        (:`3`
          (`self.SetZeroSpeed`))))
    (:`NewEnumerator1`
      ;[1 1 1] Backstep
      (bind _returnvalue_14 (`self.IncreaseToMaxInt` 1 3))
      (switch `int` _returnvalue_14
        (:`1`
          (`self.RandomInt` 1 2))
        (:`2`
          (if (not (`AnimInstance.IsAnyMontagePlaying` (`self.As ABP Boss`)))
            (bind _returnvalue_15 (`/Game/Team/KH/BP/BP_Boss.AnimBackStep` (`self.As BP Boss`)))
            (`KismetSystemLibrary.Delay` _returnvalue_15)
            (bind _returnvalue_16 (`/Game/Team/KH/BP/BP_Boss.AnimATK02` (`self.As BP Boss`)))
            (`KismetSystemLibrary.Delay` _returnvalue_16)
            (`self.ReturnToWalk`)))
        (:`3`
          (`self.SetZeroSpeed`)
          (message `/Game/Team/KH/BP/BPI_Boss.SetFocusPlayer` (`self.As Owner`)))))
    (:`NewEnumerator12`
      ;[1 1 1] Behind Attack
      (bind _returnvalue_17 (`self.IncreaseToMaxInt` 1 2))
      (switch `int` _returnvalue_17
        (:`1`
          (if (not (`AnimInstance.IsAnyMontagePlaying` (`self.As ABP Boss`)))
            (bind _returnvalue_18 (`/Game/Team/KH/BP/BP_Boss.AnimBehindATK` _as_bp_boss))
            (`KismetSystemLibrary.Delay` _returnvalue_18)
            (`self.ReturnToMoveTo`)))
        (:`2`
          (`/Game/Team/KH/BP/BP_Boss.SetFocusPlayerSpeed` _as_bp_boss 0.1))))
    (:`NewEnumerator8`
      ;[1 1 1] Guard
      (bind _returnvalue_19 (`self.IncreaseToMaxInt` 1 2))
      (switch `int` _returnvalue_19
        (:`1`
          (`/Game/Team/KH/BP/BP_Boss.GuardOrBackstepRandom` (`self.As BP Boss`)))
        (:`2`
          (`self.SetGuardMoveSpeed`))))))

(fn `GoToATK01`
  (set `self.BossStates` "NewEnumerator9")
  (set `self.SequenceValue` 0))

(fn `GoToGuard`
  (if (`/Game/Team/KH/BP/BP_Boss.IsPlayerAttack` (`self.As BP Boss`))
    (set `self.BossStates` "NewEnumerator8")
    (set `self.SequenceValue` 0)))

(fn `IncreaseToMaxInt`
  (params (Min :type Integer) (Max :type Integer))
  (returns (ReturnValue :type Integer))
  (bind _result (`/Engine/EditorBlueprintResources/StandardMacros.IncrementInt` (`self.SequenceValue`))
    (:`  `
      (return (`KismetMathLibrary.Clamp` _result Min Max)))))

(fn `RandomInt`
  (params (Min :type Integer) (Max :type Integer))
  (set `self.AttackRandomInt` (`KismetMathLibrary.RandomIntegerInRange` Min Max)))

(fn `ReturnToGuard`
  (set `self.BossStates` "NewEnumerator8")
  (set `self.SequenceValue` 0))

(fn `ReturnToMoveTo`
  (set `self.BossStates` "NewEnumerator0")
  (set `self.SequenceValue` 0))

(fn `ReturnToWalk`
  (set `self.BossStates` "NewEnumerator2")
  (set `self.SequenceValue` 0))

(fn `SetGuardMoveSpeed`
  (bind _as_bp_boss (`self.As BP Boss`))
  (if (<= (`/Game/Team/KH/BP/BP_Boss.DistanceBossToPlayer` _as_bp_boss) 400.0)
    (`/Game/Team/KH/BP/BP_Boss.SetMoveSpeed` (`self.As BP Boss`) (`KismetMathLibrary.FClamp` (- (`CharacterMovementComponent.MaxWalkSpeed` (`Character.CharacterMovement` _as_bp_boss)) 20.0) 0.0 125.0)))
  (return))

(fn `SetRunSpeed`
  (bind _as_bp_boss (`self.As BP Boss`))
  (if (<= (`/Game/Team/KH/BP/BP_Boss.DistanceBossToPlayer` _as_bp_boss) 400.0)
    (`/Game/Team/KH/BP/BP_Boss.SetMoveSpeed` _as_bp_boss (`KismetMathLibrary.FClamp` (- (`CharacterMovementComponent.MaxWalkSpeed` (`Character.CharacterMovement` _as_bp_boss)) 10.0) 0.0 700.0))
    (else
      (`/Game/Team/KH/BP/BP_Boss.SetMoveSpeed` _as_bp_boss (`KismetMathLibrary.FClamp` (+ (`CharacterMovementComponent.MaxWalkSpeed` (`Character.CharacterMovement` _as_bp_boss)) 10.0) 0.0 700.0))))
  (return))

(fn `SetWalkSpeed`
  (`/Game/Team/KH/BP/BP_Boss.SetMoveSpeed` (`self.As BP Boss`) 125.0))

(fn `SetZeroSpeed`
  (bind _as_bp_boss (`self.As BP Boss`))
  (`/Game/Team/KH/BP/BP_Boss.SetMoveSpeed` _as_bp_boss (`KismetMathLibrary.FClamp` (- (`CharacterMovementComponent.MaxWalkSpeed` (`Character.CharacterMovement` _as_bp_boss)) 10.0) 0.0 500.0)))