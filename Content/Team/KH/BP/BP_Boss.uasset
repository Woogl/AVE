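; Boss character Blueprint for a samurai-style melee enemy that reacts to hits and exposes attack, backstep, turn and focus functions.
; Point damage yaws the boss toward the hit source, then, unless super armor is on, plays a guard or normal hit montage chosen by a damage type read from HitItem.
; Tick tracks time and player distance, attack functions enable super armor, and a timeline drives slow motion.
; Several guard and movement branches are unwired or empty.
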(event `self.ReceiveAnyDamage`
  (params (Damage :type "Float (single-precision)") (DamageType :type "DamageType Object Reference") (InstigatedBy :type "Controller Object Reference") (DamageCauser :type "Actor Object Reference")))

(event `self.ReceiveBeginPlay`
  ;[1 1 1] 스폰 시
  (bind _asabp_boss (cast `/Game/Team/KH/Anim/ABP_Boss` (`SkeletalMeshComponent.GetAnimInstance` (`self.Mesh`))))
  (set `self.As ABP Boss` _asabp_boss))

(event `self.ReceivePointDamage`
  (params (Damage :type "Float (single-precision)") (DamageType :type "DamageType Object Reference") (HitLocation :type "Vector Structure") (HitNormal :type "Vector Structure") (HitComponent :type "PrimitiveComponent Object Reference") (BoneName :type Name) (ShotFromDirection :type "Vector Structure") (InstigatedBy :type "Controller Object Reference") (DamageCauser :type "Actor Object Reference") (HitInfo :type "HitResult Structure (by ref)"))
  (bind (_returnvalue_roll _returnvalue_pitch) (`KismetMathLibrary.BreakRotator` (`self.K2_GetActorRotation`)))
  (bind (_returnvalue_roll_2 _returnvalue_pitch_2 _returnvalue_yaw) (`KismetMathLibrary.BreakRotator` (`KismetMathLibrary.FindLookAtRotation` (`self.K2_GetActorLocation`) ShotFromDirection)))
  (bind _returnvalue (cast `EDamageType` (`KismetMathLibrary.Conv_IntToByte` (`.HitItem` (`GameplayStatics.BreakHitResult` HitInfo)))))
  (`self.K2_SetActorRotation` (`KismetMathLibrary.MakeRotator` _returnvalue_roll _returnvalue_pitch _returnvalue_yaw))
  (if (`self.IsSuperArmor`)
    _
    (elif (`self.IsGuarding`)
      (switch `int` (`/Game/Team/KH/Anim/ABP_Boss.ActiveChildIndex_0` (`self.As ABP Boss`))
        (:`1`
          (switch `EDamageType` _returnvalue
            (:`EDT_Standard`
              (`self.PlayAnimMontage` "/Game/Team/KH/Anim/Montage/Guard/AS_ARPG_Samurai_Anim_UE_Guard_B_Hit1_Montage.AS_ARPG_Samurai_Anim_UE_Guard_B_Hit1_Montage" 1.3))
            (:`EDT_KnockBack`
              (`self.PlayAnimMontage` "/Game/Team/KH/Anim/Montage/Guard/AS_ARPG_Samurai_Anim_UE_Guard_B_Break_Montage.AS_ARPG_Samurai_Anim_UE_Guard_B_Break_Montage"))
            (:`EDT_KnockDown`
              (`self.PlayAnimMontage` "/Game/Team/KH/Anim/Montage/Guard/AS_ARPG_Samurai_Anim_UE_Guard_B_Hit3_Montage.AS_ARPG_Samurai_Anim_UE_Guard_B_Hit3_Montage"))
            (:`EDT_KnockUp`
              (`self.PlayAnimMontage` "/Game/Team/KH/Anim/Montage/Guard/AS_ARPG_Samurai_Anim_UE_Guard_B_Hit2_Montage.AS_ARPG_Samurai_Anim_UE_Guard_B_Hit2_Montage"))))
        (:`2`
          (switch `EDamageType` _returnvalue
            (:`EDT_Standard`
              (`self.PlayAnimMontage` "/Game/Team/KH/Anim/Montage/Guard/AS_ARPG_Samurai_Anim_UE_Guard_Hit1_Montage.AS_ARPG_Samurai_Anim_UE_Guard_Hit1_Montage" 1.3))
            (:`EDT_KnockBack`
              (`self.PlayAnimMontage` "/Game/Team/KH/Anim/Montage/Guard/AS_ARPG_Samurai_Anim_UE_Guard_Break_Montage.AS_ARPG_Samurai_Anim_UE_Guard_Break_Montage"))
            (:`EDT_KnockDown`
              (`self.PlayAnimMontage` "/Game/Team/KH/Anim/Montage/Guard/AS_ARPG_Samurai_Anim_UE_Guard_Hit3_Montage.AS_ARPG_Samurai_Anim_UE_Guard_Hit3_Montage"))
            (:`EDT_KnockUp`
              (`self.PlayAnimMontage` "/Game/Team/KH/Anim/Montage/Guard/AS_ARPG_Samurai_Anim_UE_Guard_Hit2_Montage.AS_ARPG_Samurai_Anim_UE_Guard_Hit2_Montage")))))
      (else
        (switch `EDamageType` _returnvalue
          (:`EDT_Standard`
            (`self.PlayAnimMontage` "/Game/Team/Woogle/Animations/Hit/HitStandard.HitStandard"))
          (:`EDT_KnockBack`
            (`self.PlayAnimMontage` "/Game/Team/Woogle/Animations/Hit/KnockBack.KnockBack"))
          (:`EDT_KnockDown`
            (`self.PlayAnimMontage` "/Game/Team/Woogle/Animations/Hit/Anim_down_01_Montage.Anim_down_01_Montage"))
          (:`EDT_KnockUp`
            (`self.PlayAnimMontage` "/Game/Team/Woogle/Animations/Hit/GhostSamurai_APose_Hit_Up_Inplace_Montage.GhostSamurai_APose_Hit_Up_Inplace_Montage")))))))

(event `self.ReceiveTick`
  (params (DeltaSeconds :type "Float (single-precision)"))
  (bind _returnvalue (`self.K2_GetActorLocation`))
  ;[1 1 1] 실시간으로 시간&거리&각도 계산
  (`|ExecutionSequence`
    (:`then_0`
      (set `self.CurrentTime` (+ (`self.CurrentTime`) DeltaSeconds)))
    (:`then_1`
      (`self.SetDistanceToPlayer`))
    (:`then_2`
      (`KismetSystemLibrary.DrawDebugLine` _returnvalue (+ _returnvalue (* (`self.GetActorForwardVector`) 100000.0))))))

(event `WalkToLocation`)

(event `/Game/Team/KH/BP/BPI_Boss.SlowMotionBegin`
  ;[1 1 1] 슬로우 모션 함수
  (bind (_direction _slowmotiontime) (`Timeline|Timeline_0` :!via `PlayFromStart`)
    (:`Update`
      (set `self.CustomTimeDilation` _slowmotiontime))))

(event `MoveTo`)

(event `/Game/Team/KH/BP/BPI_Boss.SlowMotionEnd`
  ;[1 1 1] 슬로우 모션 함수
  (set `self.CustomTimeDilation` 1.0))

(event `/Game/Team/KH/BP/BPI_Boss.ClearFocusPlayer`
  ;[1 1 1] 포커싱 함수
  (`self.K2_SetActorRotation` (`self.K2_GetActorRotation`)))

(event `GuardSelet`)

(event `/Game/Team/KH/BP/BPI_Boss.SetFocusPlayer`
  ;[1 1 1] 포커싱 함수
)

(event `GuardMoveSpeed`
  (`self.SetGuardMoveSpeed`))

(fn `Anim Normal Attack`
  (returns (ReturnValue :type "Float (single-precision)")))

(fn `AnimATK01`
  (returns (ReturnValue :type "Float (single-precision)"))
  (set `self.IsSuperArmor` true)
  (bind _returnvalue (`self.PlayAnimMontage` "/Game/Team/KH/Anim/Montage/ATK01/AM_ATK01.AM_ATK01"))
  (return _returnvalue))

(fn `AnimATK02`
  (returns (ReturnValue :type "Float (single-precision)"))
  (set `self.IsSuperArmor` true)
  (bind _returnvalue (`self.PlayAnimMontage` "/Game/Team/KH/Anim/Montage/ATK02/AM_ATK02.AM_ATK02"))
  (return _returnvalue))

(fn `AnimBackStep`
  (returns (ReturnValue :type "Float (single-precision)"))
  (set `self.IsSuperArmor` true)
  (bind _returnvalue (`self.PlayAnimMontage` "/Game/Team/KH/Anim/Montage/Backstep/AM_Backstep.AM_Backstep"))
  (return _returnvalue))

(fn `AnimBehindATK`
  (returns (ReturnValue :type "Float (single-precision)"))
  (set `self.IsSuperArmor` true)
  (bind _returnvalue (`self.PlayAnimMontage` "/Game/Team/KH/Anim/Montage/BehindATK/AM_BehindATK.AM_BehindATK"))
  (return _returnvalue))

(fn `AnimDashAttack`
  (returns (ReturnValue :type "Float (single-precision)"))
  (set `self.IsSuperArmor` true)
  (bind _returnvalue (`self.PlayAnimMontage` "/Game/Team/KH/Anim/Montage/DashATK/AM_DashStingAttack.AM_DashStingAttack"))
  (return _returnvalue))

(fn `AnimJumpAttack`
  (returns (ReturnValue :type "Float (single-precision)"))
  (set `self.IsSuperArmor` true)
  (bind _returnvalue (`self.PlayAnimMontage` "/Game/Team/KH/Anim/Montage/JumpATK/AM_JumpAttack01.AM_JumpAttack01"))
  (return _returnvalue))

(fn `AnimLeapAttack`
  (returns (ReturnValue :type "Float (single-precision)")))

(fn `AnimStanceToLow`
  (returns (ReturnValue :type "Float (single-precision)"))
  (set `self.IsSuperArmor` true)
  (bind _returnvalue (`self.PlayAnimMontage` "/Game/Team/KH/Anim/Montage/StanceATK/AM_StanceToLowAttack.AM_StanceToLowAttack"))
  (return _returnvalue))

(fn `AnimStanceToStab`
  (returns (ReturnValue :type "Float (single-precision)"))
  (set `self.IsSuperArmor` true)
  (bind _returnvalue (`self.PlayAnimMontage` "/Game/Team/KH/Anim/Montage/StanceATK/AM_StanceToStab.AM_StanceToStab"))
  (return _returnvalue))

(fn `AnimTurnInPlace1`
  (bind _yaw (`BossAnimInstance.yaw` (`self.As ABP Boss`)))
  (bind _returnvalue (> (`KismetMathLibrary.Abs` _yaw) 135.0))
  (if (not (`AnimInstance.IsAnyMontagePlaying` (`self.As ABP Boss`)))
    (`|ExecutionSequence`
      (:`then_0`
        (if (> _yaw 70.0)
          (if _returnvalue
            (`self.PlayAnimMontage` "/Game/Team/KH/Anim/Montage/TurnInPlace/AM_Turn_Combat_180_R_Seq.AM_Turn_Combat_180_R_Seq")
            (else
              (`self.PlayAnimMontage` "/Game/Team/KH/Anim/Montage/TurnInPlace/AM_Turn_Combat_90_R_Seq.AM_Turn_Combat_90_R_Seq")))))
      (:`then_1`
        (if (< _yaw -70.0)
          (if _returnvalue
            (`self.PlayAnimMontage` "/Game/Team/KH/Anim/Montage/TurnInPlace/AM_Turn_Combat_180_L_Seq.AM_Turn_Combat_180_L_Seq")
            (else
              (`self.PlayAnimMontage` "/Game/Team/KH/Anim/Montage/TurnInPlace/AM_Turn_Combat_90_L_Seq.AM_Turn_Combat_90_L_Seq"))))))))

(fn `ApproachPlayer`)

(fn `GuardOrBackstepRandom`
  (if (<= (`self.DistanceBossToPlayer`) 400.0)
    (bind _output_get (set `self.GuardOrBackstep` (`KismetMathLibrary.RandomFloatInRange` 0.0 1.0)))
    (if (not (<= _output_get (`self.BackstepPercentage`)))
      (`self.GuardSelet`))))

(fn `SetClearFocus`
  (`self.K2_SetActorRotation` (`self.K2_GetActorRotation`)))

(fn `SetDistanceToPlayer`
  (returns (DistanceValue :type "Float (double-precision)"))
  (bind _output_get (set `self.DistanceBossToPlayer` (`KismetMathLibrary.Vector_Distance` (`self.K2_GetActorLocation`) (`self.K2_GetActorLocation` (`GameplayStatics.GetPlayerCharacter` 0)))))
  (return _output_get))

(fn `SetFocusPlayerSpeed`
  (params (Alpha :type "Float (single-precision)"))
  (bind (_returnvalue_roll _returnvalue_pitch _returnvalue_yaw) (`KismetMathLibrary.BreakRotator` (`KismetMathLibrary.RLerp` (`self.K2_GetActorRotation`) (`KismetMathLibrary.FindLookAtRotation` (`self.K2_GetActorLocation`) (`self.K2_GetActorLocation` (`GameplayStatics.GetPlayerPawn` 0))) Alpha true)))
  (`self.K2_SetActorRotation` (`KismetMathLibrary.MakeRotator` 0.0 0.0 _returnvalue_yaw)))

(fn `SetFocusPlayerTick1`
  (bind (_returnvalue_roll _returnvalue_pitch _returnvalue_yaw) (`KismetMathLibrary.BreakRotator` (`KismetMathLibrary.RLerp` (`self.K2_GetActorRotation`) (`KismetMathLibrary.FindLookAtRotation` (`self.K2_GetActorLocation`) (`self.K2_GetActorLocation` (`GameplayStatics.GetPlayerCharacter` 0))) 0.1 true)))
  (if (> (`BossAnimInstance.speed` (`self.As ABP Boss`)) 100.0)
    (`self.K2_SetActorRotation` (`KismetMathLibrary.MakeRotator` 0.0 0.0 _returnvalue_yaw))
    (else
      (`self.AnimTurnInPlace1`))))

(fn `SetGuardMoveSpeed`
  (if (<= (`self.DistanceBossToPlayer`) 400.0)
    (`self.SetMoveSpeed` (`KismetMathLibrary.FClamp` (- (`CharacterMovementComponent.MaxWalkSpeed` (`self.CharacterMovement`)) 20.0) 0.0 125.0))
    (else
      (`self.SetMoveSpeed` 125.0)))
  (return))

(fn `SetMoveSpeed`
  (params (`Max Walk Speed` :type "Float (single-precision)"))
  (returns (ReturnValue :type "Float (single-precision)"))
  (bind _output_get (set `CharacterMovementComponent.MaxWalkSpeed` `Max Walk Speed` (`self.CharacterMovement`)))
  (return _output_get))

(fn `UserConstructionScript`)