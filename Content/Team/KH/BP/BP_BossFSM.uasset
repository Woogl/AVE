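; BP_BossFSM holds movement and state logic for a boss, built around a BossStates enum.
; Live events strafe via AIMoveTo along the randomly signed right vector (without adding the boss's location), chase the player, set guard speed and print the state.
; Delay, random-direction timer and guard chains that would advance states and switch animation are disconnected, leaving their events empty.
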(event `self.IdleDelay`)

(event `self.WalkDelay`)

(event `self.SetWalkRandomInt`)

(event `self.GuardSelect`)

(event `SelectWalkRandomInt`)

(event `self.WalkToLocation`
  (params (locRange :type "Float (single-precision)"))
  (bind _asboss (`self.asBoss`))
  (bind _returnvalue (`Actor.GetActorRightVector` _asboss))
  (switch `int` (`self.walkRandomInt`)
    (:`1`
      (`|AIMoveTo` _asboss (* _returnvalue locRange) null))
    (:`2`
      (`|AIMoveTo` _asboss (* _returnvalue (* locRange -1.0)) null))))

(event `GuardMoveSpeed`
  (`self.SetGuardMoveSpeed`))

(event `self.MoveToLocation`
  (`|AIMoveTo` (`self.asBoss`) (`Actor.K2_GetActorLocation` (`GameplayStatics.GetPlayerCharacter` 0)) null))

(event `self.BossStateDebug`
  (`KismetSystemLibrary.PrintString` (`|GetEnumeratorNameAsString` (`self.bossStates`)) true true (struct :`G` 0.66 :`B` 1.0 :`A` 1.0) 0.0))