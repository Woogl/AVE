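; Player character Blueprint for boss testing, implementing Blueprint events declared in C++ alongside temporary stat UI.
; Landing briefly disables movement, longer during montages, and MotionMorph sets a motion-warp target beside the enemy for a takedown finisher, notifying Dummy targets.
; It spawns ghost trails, creates stat and screen-cut skill-effect widgets, and caches BP_Boss so a test attack input triggers its guard-or-backstep reaction at close range.
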(event `self.OnLanded`
  (params (Hit :type "HitResult Structure (by ref)"))
  ;[1 1 1] 착지
  (`CharacterMovementComponent.SetMovementMode` (`self.CharacterMovement`) "MOVE_None" 0)
  (if (`AnimInstance.IsAnyMontagePlaying` (`SkeletalMeshComponent.GetAnimInstance` (`self.Mesh`)))
    (`KismetSystemLibrary.Delay` 1.0)
    (else
      (`KismetSystemLibrary.Delay` 0.6)))
  (`CharacterMovementComponent.SetMovementMode` (`self.CharacterMovement`) "MOVE_Walking" 0))

(event `self.MotionMorph`
  (bind (_returnvalue_roll _returnvalue_pitch) (`KismetMathLibrary.BreakRotator` (`self.K2_GetActorRotation`)))
  (bind _returnvalue (`self.K2_GetActorLocation` (`self.EnemyTarget`)))
  (bind (_returnvalue_roll_2 _returnvalue_pitch_2 _returnvalue_yaw) (`KismetMathLibrary.BreakRotator` (`KismetMathLibrary.FindLookAtRotation` (`self.K2_GetActorLocation`) (`self.K2_GetActorLocation` (`self.EnemyTarget`)))))
  ;[1 1 1] 모션 워핑
  (`MotionWarpingComponent.AddOrUpdateWarpTargetFromLocationAndRotation` (`self.MotionWarping`) "TakeDown01" (+ (* (`KismetMathLibrary.Normal` (- (`self.K2_GetActorLocation`) _returnvalue)) 80.0) _returnvalue) (`KismetMathLibrary.MakeRotator` _returnvalue_roll _returnvalue_pitch _returnvalue_yaw))
  (`self.FinishEnemy`)
  (bind _asdummy (cast `Dummy` (`self.EnemyTarget`)))
  (`Dummy.OnFinishered` _asdummy))

(event `self.SpawnGhostTrail`
  ;[1 1 1] 잔상
  (`|SpawnActorFromClass` "/Game/Team/Woogle/BP_GhostTrail.BP_GhostTrail_C" (`SceneComponent.K2_GetComponentToWorld` (`self.Mesh`)) "AlwaysSpawn" "OverrideRootScale" null self null))

(event `/Game/Blueprints/BPI_Player.SetRInterpSpeed`
  (params (RInterpSpeed :type "Float (double-precision)"))
  ;[1 1 1] Anim Notify
  (set `self.RInterpSpeed` RInterpSpeed))

(event `InputAction|AttackTest`
  (params (Key :type "Key Structure"))
  (bind _as_bp_boss (`self.As BP Boss`))
  (:`Pressed`
    (if (<= (`/Game/Team/KH/BP/BP_Boss.DistanceBossToPlayer` _as_bp_boss) 400.0)
      (`BossFSMComponent.GuardOrBackstep` (`/Game/Team/KH/BP/BP_Boss.BP_BossFSM` _as_bp_boss)))))

(event `self.ReceiveBeginPlay`
  ;[1 1 1] 체력/체간 위젯(임시), 0번 스킬 반갈죽 이펙트용 위젯
  (bind _returnvalue (`|CreateWidget` "/Game/Team/Mun/WBP_PlayerStat.WBP_PlayerStat_C"))
  (bind _output_get (set `self.Widget_PlayerStat` _returnvalue))
  (`UserWidget.AddToViewport` _output_get 0)
  (bind _returnvalue_2 (`|CreateWidget` "/Game/Team/Mun/PostProcess/WBP_ScreenCut.WBP_ScreenCut_C"))
  (set `self.Widget_ScreenCut` _returnvalue_2)
  (bind _returnvalue_3 (`GameplayStatics.GetActorOfClass` "/Game/Team/KH/BP/BP_Boss.BP_Boss_C"))
  (set `self.As BP Boss` _returnvalue_3))

(fn `ScreenCut`
  (bind _widget_screencut (`self.Widget_ScreenCut`))
  (`/Game/Team/Mun/PostProcess/WBP_ScreenCut.Init` _widget_screencut)
  (`UserWidget.AddToViewport` _widget_screencut 0))

(fn `UserConstructionScript`)