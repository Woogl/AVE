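; Test player character for boss combat, with health, posture and a finisher on enemies.
; Incoming damage always drains posture, and also health unless blocking, printing both.
; An attack test input makes a nearby BP_Boss return to guard, and landing briefly disables movement, longer during montages.
; C++-declared MotionMorph uses Motion Warping to place and turn the player toward the target, runs FinishEnemy, then notifies Dummy targets.
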(event `DecreasePosture`
  (params (Damage :type "Float (double-precision)"))
  (bind _output_get (set `self.CurPosture` (- (`self.CurPosture`) Damage)))
  (`KismetSystemLibrary.PrintString` (`KismetStringLibrary.Concat_StrStr` "Posture: " (`KismetStringLibrary.Conv_DoubleToString` _output_get))))

(event `self.ReceiveAnyDamage`
  (params (Damage :type "Float (single-precision)") (DamageType :type "DamageType Object Reference") (InstigatedBy :type "Controller Object Reference") (DamageCauser :type "Actor Object Reference"))
  (if (`self.bIsBlocking`)
    (`self.DecreasePosture` Damage)
    (else
      (`self.DecreasePosture` Damage)
      (`self.DecreaseHealth` Damage))))

(event `DecreaseHealth`
  (params (Damage :type "Float (double-precision)"))
  (bind _output_get (set `self.CurHealth` (- (`self.CurHealth`) Damage)))
  (`KismetSystemLibrary.PrintString` (`KismetStringLibrary.Concat_StrStr` "Health: " (`KismetStringLibrary.Conv_DoubleToString` _output_get))))

(event `self.OnLanded`
  (params (Hit :type "HitResult Structure (by ref)"))
  ;[1 1 1] 착지
  (`CharacterMovementComponent.SetMovementMode` (`self.CharacterMovement`) "MOVE_None" 0)
  (if (`AnimInstance.IsAnyMontagePlaying` (`SkeletalMeshComponent.GetAnimInstance` (`self.Mesh`)))
    (`KismetSystemLibrary.Delay` 1.0)
    (else
      (`KismetSystemLibrary.Delay` 0.6)))
  (`CharacterMovementComponent.SetMovementMode` (`self.CharacterMovement`) "MOVE_Walking" 0))

(event `InputAction|AttackTest`
  (params (Key :type "Key Structure"))
  (:`Pressed`
    (set `self.IsAttacking` true)
    (bind _returnvalue (`GameplayStatics.GetActorOfClass` "/Game/Team/KH/BP/BP_Boss.BP_Boss_C"))
    (if (<= (`/Game/Team/KH/BP/BP_Boss.DistanceBossToPlayer` _returnvalue) 400.0)
      (`/Game/Team/KH/BP/BP_FSMComponent.ReturnToGuard` (`/Game/Team/KH/BP/BP_Boss.BP_FSMComponent` _returnvalue))
      (set `self.IsAttacking` false))))

(event `self.MotionMorph`
  (bind (_returnvalue_roll _returnvalue_pitch) (`KismetMathLibrary.BreakRotator` (`self.K2_GetActorRotation`)))
  (bind _returnvalue (`self.K2_GetActorLocation` (`self.EnemyTarget`)))
  (bind (_returnvalue_roll_2 _returnvalue_pitch_2 _returnvalue_yaw) (`KismetMathLibrary.BreakRotator` (`KismetMathLibrary.FindLookAtRotation` (`self.K2_GetActorLocation`) (`self.K2_GetActorLocation` (`self.EnemyTarget`)))))
  ;[1 1 1] 모션 워핑
  (`MotionWarpingComponent.AddOrUpdateWarpTargetFromLocationAndRotation` (`self.MotionWarping`) "TakeDown01" (+ (* (`KismetMathLibrary.Normal` (- (`self.K2_GetActorLocation`) _returnvalue)) 80.0) _returnvalue) (`KismetMathLibrary.MakeRotator` _returnvalue_roll _returnvalue_pitch _returnvalue_yaw))
  (`self.FinishEnemy`)
  (bind _asdummy (cast `Dummy` (`self.EnemyTarget`)))
  (`Dummy.OnFinishered` _asdummy))

(event `/Game/Blueprints/BPI_Player.SetRInterpSpeed`
  (params (RInterpSpeed :type "Float (double-precision)"))
  ;[1 1 1] Anim Notify
  (set `self.RInterpSpeed` RInterpSpeed))

(fn `UserConstructionScript`)