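; Tutorial sliding double door that stays locked until its StageCleared event sets CanOpen.
; Once unlocked, overlapping the Box trigger plays a click sound and runs two timelines that slide the Left and Right panels apart along Y.
; Leaving the trigger plays a back-click sound and reverses both timelines to close it.
; The construction script scales the actor's width and height from UnitSize to fit the opening.
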(event `/Game/Team/Woogle/BPI_CardKeyDoor.StageCleared`
  (set `self.bCanOpen` true))

(event `self.Box.OnComponentBeginOverlap`
  (params (OverlappedComponent :type "PrimitiveComponent Object Reference") (OtherActor :type "Actor Object Reference") (OtherComp :type "PrimitiveComponent Object Reference") (OtherBodyIndex :type Integer) (bFromSweep :type Boolean) (SweepResult :type "HitResult Structure (by ref)"))
  (if (`self.bCanOpen`)
    ;[1 1 1] TODO : Set door slide sound
    (`GameplayStatics.SpawnSoundAtLocation` "/Game/MarketplaceAssets/Interface_And_Item_Sounds/Cues/Click_07_Cue.Click_07_Cue" (`self.K2_GetActorLocation`) (struct) 1.0 1.0 0.0 null null)
    (`|ExecutionSequence`
      (:`then_0`
        (bind (_direction _alpha) (`Timeline|Timeline_0` :!label _label)
          (:`Update`
            (`SceneComponent.K2_SetRelativeLocation` (`self.Left`) (`KismetMathLibrary.MakeVector` 0.0 (`KismetMathLibrary.Lerp` 0.0 130.0 _alpha)) false false))))
      (:`then_1`
        (bind (_direction_2 _alpha_2) (`Timeline|Timeline_1` :!label _label_2)
          (:`Update`
            (`SceneComponent.K2_SetRelativeLocation` (`self.Right`) (`KismetMathLibrary.MakeVector` 0.0 (`KismetMathLibrary.Lerp` 0.0 -130.0 _alpha_2)) false false)))))))

(event `self.Box.OnComponentEndOverlap`
  (params (OverlappedComponent :type "PrimitiveComponent Object Reference") (OtherActor :type "Actor Object Reference") (OtherComp :type "PrimitiveComponent Object Reference") (OtherBodyIndex :type Integer))
  (if (`self.bCanOpen`)
    ;[1 1 1] TODO : Set door slide sound
    (`GameplayStatics.SpawnSoundAtLocation` "/Game/MarketplaceAssets/Interface_And_Item_Sounds/Cues/Back_Click_07_Cue.Back_Click_07_Cue" (`self.K2_GetActorLocation`) (struct) 1.0 1.0 0.0 null null)
    (`|ExecutionSequence`
      (:`then_0`
        (goto _label :!via `Reverse`))
      (:`then_1`
        (goto _label_2 :!via `Reverse`)))))

(fn `UserConstructionScript`
  (bind (_unitsize_x _unitsize_y _unitsize_z) (`KismetMathLibrary.BreakVector` (`self.UnitSize`)))
  (`self.SetActorScale3D` (`KismetMathLibrary.MakeVector` 1.0 (/ _unitsize_y 286.0) (/ _unitsize_z 436.0))))