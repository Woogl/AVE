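; BP_Locker is a locker prop that dresses itself with two randomly placed books when its construction script runs.
; The script rolls one of five shelf heights for each book, looping until the second differs from the first.
; ChangeBookState then gives each book a random material, per-axis scale, position along the shelf and upright or sideways roll.
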(fn `Change Book State`
  (params (BookToChange :type "PrimitiveComponent Object Reference") (FloorIndex :type Integer))
  (bind _returnvalue (`KismetMathLibrary.RandomFloatInRange` 0.6 0.95))
  (`PrimitiveComponent.SetMaterial` BookToChange 0 (`KismetArrayLibrary.Array_Random` (`self.BookMat`)))
  (`SceneComponent.SetRelativeScale3D` BookToChange (`KismetMathLibrary.MakeVector` _returnvalue _returnvalue _returnvalue))
  (`SceneComponent.K2_SetRelativeLocationAndRotation` BookToChange (`KismetMathLibrary.MakeVector` -40.0 (`KismetMathLibrary.RandomFloatInRange` -160.0 -30.0) (select `int` FloorIndex :`0` 4.0 :`1` 44.0 :`2` 82.0 :`3` 124.0 :`4` 162.0)) (`KismetMathLibrary.MakeRotator` (`KismetMathLibrary.SelectFloat` 0.0 -90.0 (`KismetMathLibrary.RandomBool`))) false false))

(fn `UserConstructionScript`
  (locals (selected1 :type Integer :default 0) (selected2 :type Integer :default 0))
  (`|ExecutionSequence`
    (:`then_0`
      (set `local.selected1` (`KismetMathLibrary.RandomIntegerInRange` 0 4))
      (`self.Change Book State` (`self.Book1`) (`local.selected1`)))
    (:`then_1`
      (set `local.selected2` (`KismetMathLibrary.RandomIntegerInRange` 0 4) :!label _label)
      (if (== (`local.selected1`) (`local.selected2`))
        (goto _label)
        (else
          (`self.Change Book State` (`self.Book2`) (`local.selected2`)))))))