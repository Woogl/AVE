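; BP_Lobby is a building interior stage that lays out a fixed lobby template on an indexed grid and offsets its stage start trigger.
; SpawnTemplate places four columns at the grid corners, or inset when Width is at least seven, then a parity-adjusted centerpiece ringed by four rotated sliceable desks.
; It spawns three randomly facing swordsmen relative to the center and column indices, linking each to this interior and setting the enemy count.
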(fn `CustomStageStartEvent`)

(fn `RelocateComp`
  (params (Comp :type "SceneComponent Object Reference"))
  (`parent.RelocateComp` Comp))

(fn `SpawnTemplate`
  (locals (centerIndex :type Integer :default 0) (firstColumnIndex :type Integer) (thirdColumnIndex :type Integer))
  (bind _returnvalue (+ (`self.Depth`) 1))
  (bind _returnvalue_2 (- (* (`self.Depth`) (`self.Width`)) (`self.Depth`) 2))
  (bind _returnvalue_3 (- (* (`self.Depth`) (`self.Width`)) 1))
  (bind _returnvalue_4 (/ (* (`self.Width`) (`self.Depth`)) 2))
  (bind _returnvalue_5 (- _returnvalue_2 (- (`self.Depth`) 3)))
  (`|ExecutionSequence`
    (:`then_0`
      (if (< (`self.Width`) 7)
        (`|SpawnActorFromClass` "/Game/Team/Woogle/Building/BP_LobbyColumn.BP_LobbyColumn_C" (`KismetMathLibrary.MakeTransform` (`self.ConvertIndexToLoc` 0)) "AdjustIfPossibleButAlwaysSpawn" "OverrideRootScale" null null)
        (set `local.firstColumnIndex` 0)
        (`|SpawnActorFromClass` "/Game/Team/Woogle/Building/BP_LobbyColumn.BP_LobbyColumn_C" (`KismetMathLibrary.MakeTransform` (`self.ConvertIndexToLoc` (- (`self.Depth`) 1))) "AdjustIfPossibleButAlwaysSpawn" "OverrideRootScale" null null)
        (`|SpawnActorFromClass` "/Game/Team/Woogle/Building/BP_LobbyColumn.BP_LobbyColumn_C" (`KismetMathLibrary.MakeTransform` (`self.ConvertIndexToLoc` _returnvalue_3)) "AdjustIfPossibleButAlwaysSpawn" "OverrideRootScale" null null)
        (set `local.thirdColumnIndex` _returnvalue_3)
        (`|SpawnActorFromClass` "/Game/Team/Woogle/Building/BP_LobbyColumn.BP_LobbyColumn_C" (`KismetMathLibrary.MakeTransform` (`self.ConvertIndexToLoc` (- _returnvalue_3 -1 (`self.Depth`)))) "AdjustIfPossibleButAlwaysSpawn" "OverrideRootScale" null null)
        (else
          (`|SpawnActorFromClass` "/Game/Team/Woogle/Building/BP_LobbyColumn.BP_LobbyColumn_C" (`KismetMathLibrary.MakeTransform` (`self.ConvertIndexToLoc` _returnvalue)) "AdjustIfPossibleButAlwaysSpawn" "OverrideRootScale" null null)
          (set `local.firstColumnIndex` _returnvalue)
          (`|SpawnActorFromClass` "/Game/Team/Woogle/Building/BP_LobbyColumn.BP_LobbyColumn_C" (`KismetMathLibrary.MakeTransform` (`self.ConvertIndexToLoc` (+ _returnvalue (- (`self.Depth`) 3)))) "AdjustIfPossibleButAlwaysSpawn" "OverrideRootScale" null null)
          (`|SpawnActorFromClass` "/Game/Team/Woogle/Building/BP_LobbyColumn.BP_LobbyColumn_C" (`KismetMathLibrary.MakeTransform` (`self.ConvertIndexToLoc` _returnvalue_2)) "AdjustIfPossibleButAlwaysSpawn" "OverrideRootScale" null null)
          (`|SpawnActorFromClass` "/Game/Team/Woogle/Building/BP_LobbyColumn.BP_LobbyColumn_C" (`KismetMathLibrary.MakeTransform` (`self.ConvertIndexToLoc` _returnvalue_5)) "AdjustIfPossibleButAlwaysSpawn" "OverrideRootScale" null null)
          (set `local.thirdColumnIndex` _returnvalue_5))))
    (:`then_1`
      (bind _output_get (set `local.centerIndex` (`KismetMathLibrary.SelectInt` _returnvalue_4 (+ _returnvalue_4 (/ (`self.Depth`) 2)) (`KismetMathLibrary.Conv_IntToBool` (mod (`self.Width`) 2)))))
      (`|SpawnActorFromClass` "/Game/Team/Woogle/Building/BP_LobbyCenter.BP_LobbyCenter_C" (`KismetMathLibrary.MakeTransform` (`self.ConvertIndexToLoc` _output_get)) "AdjustIfPossibleButAlwaysSpawn" "OverrideRootScale" null null))
    (:`then_2`
      (`|SpawnActorFromClass` "/Game/Team/Woogle/Building/BP_SliceableDesk.BP_SliceableDesk_C" (`KismetMathLibrary.MakeTransform` (`self.ConvertIndexToLoc` (- (`local.centerIndex`) (`self.Depth`)))) "AdjustIfPossibleButAlwaysSpawn" "OverrideRootScale" null null)
      (`|SpawnActorFromClass` "/Game/Team/Woogle/Building/BP_SliceableDesk.BP_SliceableDesk_C" (`KismetMathLibrary.MakeTransform` (`self.ConvertIndexToLoc` (+ (`local.centerIndex`) (`self.Depth`))) (struct :`Yaw` 180.0)) "AdjustIfPossibleButAlwaysSpawn" "OverrideRootScale" null null)
      (`|SpawnActorFromClass` "/Game/Team/Woogle/Building/BP_SliceableDesk.BP_SliceableDesk_C" (`KismetMathLibrary.MakeTransform` (`self.ConvertIndexToLoc` (- (`local.centerIndex`) 1 (* (`self.Depth`) -1))) (struct :`Yaw` 90.0)) "AdjustIfPossibleButAlwaysSpawn" "OverrideRootScale" null null)
      (`|SpawnActorFromClass` "/Game/Team/Woogle/Building/BP_SliceableDesk.BP_SliceableDesk_C" (`KismetMathLibrary.MakeTransform` (`self.ConvertIndexToLoc` (+ (`local.centerIndex`) 1 (* (`self.Depth`) -1))) (struct :`Yaw` -90.0)) "AdjustIfPossibleButAlwaysSpawn" "OverrideRootScale" null null))
    (:`then_3`
      (`|SpawnActorFromClass` "/Game/Team/TH/Blueprints/BP_Swordman.BP_Swordman_C" (`KismetMathLibrary.MakeTransform` (`self.ConvertIndexToLoc` (- (`local.centerIndex`) 2)) (`KismetMathLibrary.MakeRotator` 0.0 0.0 (`KismetMathLibrary.RandomFloatInRange` 0.0 360.0))) "AdjustIfPossibleButAlwaysSpawn" "OverrideRootScale" null 9 self null)
      (`|SpawnActorFromClass` "/Game/Team/TH/Blueprints/BP_Swordman.BP_Swordman_C" (`KismetMathLibrary.MakeTransform` (`self.ConvertIndexToLoc` (+ (`local.firstColumnIndex`) 2)) (`KismetMathLibrary.MakeRotator` 0.0 0.0 (`KismetMathLibrary.RandomFloatInRange` 0.0 360.0))) "AdjustIfPossibleButAlwaysSpawn" "OverrideRootScale" null 9 self null)
      (`|SpawnActorFromClass` "/Game/Team/TH/Blueprints/BP_Swordman.BP_Swordman_C" (`KismetMathLibrary.MakeTransform` (`self.ConvertIndexToLoc` (+ (`local.thirdColumnIndex`) 2)) (`KismetMathLibrary.MakeRotator` 0.0 0.0 (`KismetMathLibrary.RandomFloatInRange` 0.0 360.0))) "AdjustIfPossibleButAlwaysSpawn" "OverrideRootScale" null 9 self null)
      (set `self.CurEnemyNum` 3))))

(fn `UserConstructionScript`
  (locals (NewWallSacle :type "Vector Structure" :default (0.0 0.0 0.0)) (doorIndex :type Integer :default 0))
  (`parent.UserConstructionScript`)
  (`SceneComponent.K2_SetRelativeLocationAndRotation` :`self` (`self.StageStartTrigger`) :`NewLocation` (0.0 -5000.0 -200.0)))