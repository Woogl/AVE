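; Base actor for one building floor's interior, running a combat stage that signals the elevator when its last enemy dies.
; Construction builds a randomly styled instanced floor grid and records cell indices.
; The start trigger clears old enemies, optionally calls the empty SpawnTemplate hook, then uses shuffled cells for height-scaled swordsmen and wall-aware props before refreshing the AI manager.
; The end trigger destroys the interior.
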(event `self.StageStartTrigger.OnComponentBeginOverlap`
  (params (OverlappedComponent :type "PrimitiveComponent Object Reference") (OtherActor :type "Actor Object Reference") (OtherComp :type "PrimitiveComponent Object Reference") (OtherBodyIndex :type Integer) (bFromSweep :type Boolean) (SweepResult :type "HitResult Structure (by ref)"))
  (bind _aimanagerref (`/Game/Team/Woogle/Building/BP_BuildingManager.AIManagerRef` (`self.BuildingManagerRef`)))
  (`/Engine/EditorBlueprintResources/StandardMacros.DoOnce` false
    (:`Completed`
      (bind _outactors (`GameplayStatics.GetAllActorsOfClass` "/Script/AVE.EnemyBase"))
      (for _array_element _outactors
        (`self.K2_DestroyActor` _array_element))
      (`|ExecutionSequence`
        (:`then_0`
          (if (`self.bIsTemplateStage`)
            (`self.SpawnTemplate`))
          (`KismetArrayLibrary.Array_Shuffle` (`self.LocIndexes`)))
        (:`then_1`
          (if (`self.bCanSpawnRandomEnemies`)
            (set `self.MaxEnemyNum` (+ (`self.CurHeight`) 2))
            (for _index (range (`self.MaxEnemyNum`))
              (`|SpawnActorFromClass` "/Game/Team/TH/Blueprints/BP_Swordman.BP_Swordman_C" (`KismetMathLibrary.MakeTransform` (`self.ConvertIndexToLoc` (`|GetArrayItem` (`self.LocIndexes`) _index)) (`KismetMathLibrary.MakeRotator` 0.0 0.0 (`KismetMathLibrary.RandomFloatInRange` 0.0 360.0))) "AdjustIfPossibleButAlwaysSpawn" "OverrideRootScale" null 9 self null)
              (`/Engine/EditorBlueprintResources/StandardMacros.IncrementInt` (`self.CurEnemyNum`)))))
        (:`then_2`
          (if (`self.bCanSpawnProps`)
            (for _index_2 (range (`self.MaxEnemyNum`) (+ (+ (`self.MaxEnemyNum`) (`self.PropNum`) -1) 1))
              (`self.SpawnRandomProp` (`|GetArrayItem` (`self.LocIndexes`) _index_2)))))
        (:`then_3`
          (`KismetArrayLibrary.Array_Clear` (`AIManager.Enemies` _aimanagerref))
          (`KismetSystemLibrary.Delay` 0.5)
          (`AIManager.EnemySearch` _aimanagerref)
          (if (!= (`self.CurHeight`) 1)
            (`AIManager.RunAI` _aimanagerref)))))))

(event `self.StageEndTrigger.OnComponentBeginOverlap`
  (params (OverlappedComponent :type "PrimitiveComponent Object Reference") (OtherActor :type "Actor Object Reference") (OtherComp :type "PrimitiveComponent Object Reference") (OtherBodyIndex :type Integer) (bFromSweep :type Boolean) (SweepResult :type "HitResult Structure (by ref)"))
  (`/Engine/EditorBlueprintResources/StandardMacros.DoOnce` false
    (:`Completed`
      (`self.K2_DestroyActor`))))

(event `/Game/Team/Woogle/Building/BPI_Building.OnEnemyDie`
  (bind _buildingelements (`/Game/Team/Woogle/Building/BP_BuildingManager.BuildingElements` (`self.BuildingManagerRef`)))
  (bind _result (`/Engine/EditorBlueprintResources/StandardMacros.DecrementInt` (`self.CurEnemyNum`))
    (:`  `
      (if (== _result 0)
        (message `/Game/Team/Woogle/Building/BPI_Building.OnStageWin` (`|GetArrayItem` _buildingelements (`KismetArrayLibrary.Array_LastIndex` _buildingelements)))))))

(fn `ConvertIndexToLoc`
  (params (Index :type Integer))
  (returns (ReturnValue :type "Vector Structure"))
  (bind _depth (`self.Depth`))
  (bind (_unitsize_x _unitsize_y) (`KismetMathLibrary.BreakVector` (`self.UnitSize`)))
  (bind (_unitsize_x_2 _unitsize_y_2) (`KismetMathLibrary.BreakVector` (`self.UnitSize`)))
  (return (+ (`KismetMathLibrary.MakeVector` (+ (* (/ Index _depth) _unitsize_x) (* (`self.Width`) _unitsize_x_2 -0.5) (* _unitsize_x_2 0.5)) (+ (* (mod Index _depth) _unitsize_y) (* _unitsize_y_2 0.5))) (`self.K2_GetActorLocation`))))

(fn `RelocateComp`
  (params (Comp :type "SceneComponent Object Reference"))
  (bind _unitsize_x (`KismetMathLibrary.BreakVector` (`self.UnitSize`)))
  (`SceneComponent.K2_SetRelativeLocation` Comp (`KismetMathLibrary.MakeVector` (* _unitsize_x (`self.Width`) -0.5)) false false))

(fn `SpawnRandomProp`
  (params (Index :type Integer))
  (locals (spawnRot :type "Rotator Structure") (selectedIndex :type Integer :default 0))
  (bind _returnvalue (mod Index (`self.Depth`)))
  ;[0 0 0] 인덱스 = 벽
  (if (< Index (`self.Depth`))
    (set `local.spawnRot` (struct))
    (`|SpawnActorFromClass` (`|GetArrayItem` (`self.WallProps`)) (`KismetMathLibrary.MakeTransform` (`self.ConvertIndexToLoc` Index) (`local.spawnRot`)) "AdjustIfPossibleButAlwaysSpawn" "OverrideRootScale" null null :!label _label)
    (elif (> Index (- (* (`self.Depth`) (`self.Width`)) (`self.Depth`)))
      (set `local.spawnRot` (struct :`Yaw` 180.0))
      (goto _label)
      (elif (== _returnvalue 0)
        (set `local.spawnRot` (struct :`Yaw` 90.0))
        (goto _label)
        (elif (== _returnvalue (- (`self.Depth`) 1))
          (set `local.spawnRot` (struct :`Yaw` -90.0))
          (goto _label)
          (else
            ;[0 0 0] 인덱스 != 벽
            (`|SpawnActorFromClass` (`KismetArrayLibrary.Array_Random` (`self.GroundProps`)) (`KismetMathLibrary.MakeTransform` (`self.ConvertIndexToLoc` Index) (`KismetMathLibrary.MakeRotator` 0.0 0.0 (`KismetMathLibrary.RandomFloatInRange` 0.0 360.0))) "AdjustIfPossibleButAlwaysSpawn" "OverrideRootScale" null null)))))))

(fn `SpawnTemplate`)

(fn `UserConstructionScript`
  (locals (NewWallSacle :type "Vector Structure" :default (0.0 0.0 0.0)) (doorIndex :type Integer :default 0))
  (bind (_unitsize_x _unitsize_y) (`KismetMathLibrary.BreakVector` (`self.UnitSize`)))
  (bind _indexselector (`self.IndexSelector`))
  (bind _floorinstance (`self.FloorInstance`))
  (bind (_unitsize_x_2 _unitsize_y_2 _unitsize_z) (`KismetMathLibrary.BreakVector` (`self.UnitSize`)))
  (bind (_unitsize_x_3 _unitsize_y_3) (`KismetMathLibrary.BreakVector` (`self.UnitSize`)))
  (bind _returnvalue (* _unitsize_y_3 (+ (`self.Depth`) 1)))
  (`|ExecutionSequence`
    (:`then_0`
      ;[0 0 0] Floor
      (`PrimitiveComponent.SetMaterial` (`self.FloorInstance`) 0 (`KismetArrayLibrary.Array_Random` (`self.RandomMaterials`)))
      (if (`self.bRandomUnderLighit`)
        (`MeshComponent.SetVectorParameterValueOnMaterials` (`self.FloorInstance`) "emissiveColor" (`KismetMathLibrary.MakeVector` (`KismetMathLibrary.RandomFloatInRange` 0.0 1.0) (`KismetMathLibrary.RandomFloatInRange` 0.0 1.0) (`KismetMathLibrary.RandomFloatInRange` 0.0 1.0))))
      (for _index (range (`self.Width`))
        (for _index_2 (range (`self.Depth`))
          (`InstancedStaticMeshComponent.AddInstance` _floorinstance (`KismetMathLibrary.MakeTransform` (`KismetMathLibrary.MakeVector` (* _unitsize_x _index) (* _unitsize_y _index_2)) (struct) (1.0 0.91 1.0)) false)
          (`self.RelocateComp` _floorinstance)
          (`KismetArrayLibrary.Array_Add` (`self.LocIndexes`) _indexselector)
          (bind _result (`/Engine/EditorBlueprintResources/StandardMacros.IncrementInt` _indexselector)))))
    (:`then_1`
      ;[0 0 0] Stage Trigger
      (`SceneComponent.K2_SetRelativeLocation` (`self.StageStartTrigger`) (`KismetMathLibrary.MakeVector` 0.0 _returnvalue) false false)
      (`SceneComponent.K2_SetRelativeLocation` (`self.StageEndTrigger`) (`KismetMathLibrary.MakeVector` 0.0 _returnvalue (* _unitsize_z 1.42)) false false))))