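; BP_RoofTop is a rooftop boss stage sized by Width, Depth and UnitSize.
; The construction script rings it with scaled fence instances, leaves a gap mid-way along one Width edge, scales a heliport decal and positions three blockers.
; On stage start it spawns BP_Boss with a controller at mid-depth, switches the BGM through the game mode and sets the neon sign's emissive strength.
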(fn `CustomStageStartEvent`
  (bind (_unitsize_x _unitsize_y) (`KismetMathLibrary.BreakVector` (`self.UnitSize`)))
  (bind _returnvalue (`|SpawnActorFromClass` "/Game/Team/KH/BP/BP_Boss.BP_Boss_C" (`KismetMathLibrary.MakeTransform` (+ (`self.K2_GetActorLocation`) (`KismetMathLibrary.MakeVector` 0.0 (* (`self.Depth`) _unitsize_y 0.5) 200.0))) "AdjustIfPossibleButAlwaysSpawn" "OverrideRootScale" null null))
  (`Pawn.SpawnDefaultController` _returnvalue)
  (bind _asavegame_mode_base (cast `AVEGameModeBase` (`GameplayStatics.GetGameMode`)))
  (`AVEGameModeBase.PlayBGM` _asavegame_mode_base "/Game/Team/Woogle/Sounds/DeathLoop3_Cue.DeathLoop3_Cue")
  (`MeshComponent.SetScalarParameterValueOnMaterials` (`self.KB3D_CBP_Hypergear_A_NeonSign`) "emissive_mult" 0.5))

(fn `UserConstructionScript`
  (bind (_unitsize_x _unitsize_y) (`KismetMathLibrary.BreakVector` (`self.UnitSize`)))
  (bind _decal (`self.Decal`))
  (bind (_unitsize_x_2 _unitsize_y_2) (`KismetMathLibrary.BreakVector` (`self.UnitSize`)))
  (bind (_unitsize_x_3 _unitsize_y_3 _unitsize_z) (`KismetMathLibrary.BreakVector` (`self.UnitSize`)))
  (bind (_unitsize_x_4 _unitsize_y_4) (`KismetMathLibrary.BreakVector` (`self.UnitSize`)))
  (bind _unitsize_x_5 (`KismetMathLibrary.BreakVector` (`self.UnitSize`)))
  (bind (_unitsize_x_6 _unitsize_y_5) (`KismetMathLibrary.BreakVector` (`self.UnitSize`)))
  (bind _unitsize_x_7 (`KismetMathLibrary.BreakVector` (`self.UnitSize`)))
  (bind (_unitsize_x_8 _unitsize_y_6) (`KismetMathLibrary.BreakVector` (`self.UnitSize`)))
  (bind (_min _max) (`StaticMeshComponent.GetLocalBounds` (`self.FenceInstance`)))
  (bind _returnvalue (* (`self.Width`) _unitsize_x_7 0.5))
  (bind _returnvalue_2 (`KismetMathLibrary.Conv_IntToDouble` (`KismetMathLibrary.Min` (`self.Width`) (`self.Depth`))))
  (bind _returnvalue_3 (`KismetMathLibrary.FMax` (.x _max) (.y _max)))
  (`parent.UserConstructionScript`)
  (`|ExecutionSequence`
    (:`then_0`
      ;[0 0 0] Left Fence
      (set `self.NewFenceScale` (`KismetMathLibrary.MakeVector` (/ _unitsize_x_3 _returnvalue_3) (/ _unitsize_y_3 _returnvalue_3) (/ _unitsize_z (* (.z _max) 2.0))))
      (`self.RelocateComp` (`self.FenceInstance`))
      (for _index (range (`self.Depth`))
        (`InstancedStaticMeshComponent.AddInstance` (`self.FenceInstance`) (`KismetMathLibrary.MakeTransform` (`KismetMathLibrary.MakeVector` (* _unitsize_x (`self.Width`)) (* _unitsize_y _index)) (struct) (`self.NewFenceScale`)) false)))
    (:`then_1`
      ;[0 0 0] Right Fence
      (for _index_2 (range (`self.Depth`))
        (`InstancedStaticMeshComponent.AddInstance` (`self.FenceInstance`) (`KismetMathLibrary.MakeTransform` (`KismetMathLibrary.MakeVector` 0.0 (* _unitsize_y_2 (+ _index_2 1))) (struct :`Yaw` 180.0) (`self.NewFenceScale`)) false)))
    (:`then_2`
      ;[0 0 0] Forward Fence
      (for _index_3 (range (`self.Width`))
        (`InstancedStaticMeshComponent.AddInstance` (`self.FenceInstance`) (`KismetMathLibrary.MakeTransform` (`KismetMathLibrary.MakeVector` (* _unitsize_x_5 _index_3)) (struct :`Yaw` -90.0) (`self.NewFenceScale`)) false)))
    (:`then_3`
      ;[0 0 0] Backward Fence
      (for _index_4 (range (`self.Width`))
        (if (not (== _index_4 (/ (`self.Width`) 2)))
          (`InstancedStaticMeshComponent.AddInstance` (`self.FenceInstance`) (`KismetMathLibrary.MakeTransform` (`KismetMathLibrary.MakeVector` (* _unitsize_x_6 (+ _index_4 1)) (* _unitsize_y_5 (`self.Depth`))) (struct :`Yaw` 90.0) (`self.NewFenceScale`)) false))))
    (:`then_4`
      ;[0 0 0] Heliport Decal
      (`SceneComponent.K2_SetRelativeLocation` _decal (`KismetMathLibrary.MakeVector` 0.0 (* (`self.Depth`) _unitsize_y_6 0.5)) false false)
      (`SceneComponent.SetRelativeScale3D` _decal (`KismetMathLibrary.MakeVector` 1.0 _returnvalue_2 _returnvalue_2)))
    (:`then_5`
      (`SceneComponent.K2_SetRelativeLocationAndRotation` :`self` (`self.BlockF`) :`NewLocation` (`KismetMathLibrary.MakeVector` 0.0 (* (`self.Depth`) _unitsize_y_4) 1024.0))
      (`SceneComponent.K2_SetRelativeLocationAndRotation` (`self.BlockL`) (`KismetMathLibrary.MakeVector` _returnvalue 0.0 1024.0) (struct :`Yaw` 90.0) false false)
      (`SceneComponent.K2_SetRelativeLocationAndRotation` (`self.BlockR`) (`KismetMathLibrary.MakeVector` (* _returnvalue -1.0) 0.0 1024.0) (struct :`Yaw` -90.0) false false))))