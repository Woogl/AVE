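; BP_Infrastructure is a building Blueprint that lays out fencing around a large rectangular area.
; Its construction script uses four loops to add evenly spaced instances to the Fence instanced mesh component.
; Two short runs share one edge with a gap between them, and two long rotated runs form the perpendicular sides.
; The script places no fence on the far edge, and all offsets are hardcoded.
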(fn `UserConstructionScript`
  (for _index (range 9)
    (`InstancedStaticMeshComponent.AddInstance` (`self.Fence`) (`KismetMathLibrary.MakeTransform` (`KismetMathLibrary.MakeVector` 0.0 (+ (* _index -200.0) -5.0))) false))
  (for _index_2 (range 9)
    (`InstancedStaticMeshComponent.AddInstance` (`self.Fence`) (`KismetMathLibrary.MakeTransform` (`KismetMathLibrary.MakeVector` -15.0 (+ (* _index_2 200.0) -5590.0)) (struct :`Yaw` 180.0)) false))
  (for _index_3 (range 25)
    (`InstancedStaticMeshComponent.AddInstance` (`self.Fence`) (`KismetMathLibrary.MakeTransform` (`KismetMathLibrary.MakeVector` (+ (* _index_3 -200.0) -9.0) 200.0) (struct :`Yaw` 90.0)) false))
  (for _index_4 (range 25)
    (`InstancedStaticMeshComponent.AddInstance` (`self.Fence`) (`KismetMathLibrary.MakeTransform` (`KismetMathLibrary.MakeVector` (+ (* _index_4 -200.0) -10.0) -5785.0) (struct :`Yaw` 90.0)) false)))