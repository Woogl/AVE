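; BP_FrontDoor is an automatic double sliding door that opens on overlap with its Box trigger and closes when the overlap ends.
; Separate DoorLeft and DoorRight timelines play or reverse to slide the Left and Right meshes along local Y.
; The construction script rescales the whole actor in Y and Z, fitting it to a UnitSize using the Right mesh's local bounds.
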(event `self.Box.OnComponentBeginOverlap`
  (params (OverlappedComponent :type "PrimitiveComponent Object Reference") (OtherActor :type "Actor Object Reference") (OtherComp :type "PrimitiveComponent Object Reference") (OtherBodyIndex :type Integer) (bFromSweep :type Boolean) (SweepResult :type "HitResult Structure (by ref)"))
  (`|ExecutionSequence`
    (:`then_0`
      (bind (_direction _left) (`Timeline|DoorLeft` :!label _label)
        (:`Update`
          (`SceneComponent.K2_SetRelativeLocation` (`self.Left`) (`KismetMathLibrary.MakeVector` 0.0 _left) false false))))
    (:`then_1`
      (bind (_direction_2 _right) (`Timeline|DoorRight` :!label _label_2)
        (:`Update`
          (`SceneComponent.K2_SetRelativeLocation` (`self.Right`) (`KismetMathLibrary.MakeVector` 0.0 _right) false false))))))

(event `self.Box.OnComponentEndOverlap`
  (params (OverlappedComponent :type "PrimitiveComponent Object Reference") (OtherActor :type "Actor Object Reference") (OtherComp :type "PrimitiveComponent Object Reference") (OtherBodyIndex :type Integer))
  (`|ExecutionSequence`
    (:`then_0`
      (goto _label :!via `Reverse`))
    (:`then_1`
      (goto _label_2 :!via `Reverse`))))

(fn `UserConstructionScript`
  (bind (_unitsize_x _unitsize_y _unitsize_z) (`KismetMathLibrary.BreakVector` (`self.UnitSize`)))
  (bind (_min _max) (`StaticMeshComponent.GetLocalBounds` (`self.Right`)))
  (`self.SetActorScale3D` (`KismetMathLibrary.MakeVector` 1.0 (/ _unitsize_y (* (.y _max) 2.0)) (/ _unitsize_z (.z _max)))))