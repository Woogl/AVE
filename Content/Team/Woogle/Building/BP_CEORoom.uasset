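; CEO office room, a child of a room Blueprint, that overrides SpawnTemplateProps to furnish a fixed, grid-based layout.
; It computes a center cell from Width and Depth, adjusted for odd or even width, then places two conference desks, the CEO desk and its back piece around it.
; Index math also puts columns at the corners and lockers flanking wall shelves on two opposite edges.
; All other overridden functions just call the parent.
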(fn `RelocateComp`
  (params (Comp :type "SceneComponent Object Reference"))
  (`parent.RelocateComp` Comp))

(fn `SpawnRandomEnemy`
  (`parent.SpawnRandomEnemy`))

(fn `SpawnRandomProp`
  (`parent.SpawnRandomProp`))

(fn `SpawnTemplateProps`
  (locals (centerIndex :type Integer :default 0))
  (bind _returnvalue (- (* (`self.Depth`) (`self.Width`)) 1))
  (bind _returnvalue_2 (/ (* (`self.Width`) (`self.Depth`)) 2))
  (`|ExecutionSequence`
    (:`then_0`
      (bind _output_get (set `local.centerIndex` (`KismetMathLibrary.SelectInt` _returnvalue_2 (+ _returnvalue_2 (/ (`self.Depth`) 2)) (`KismetMathLibrary.Conv_IntToBool` (mod (`self.Width`) 2)))))
      (`self.SpawnActorAtIndex` "/Game/Team/Woogle/Building/BP_SliceableConfDesk.BP_SliceableConfDesk_C" (+ _output_get (`self.Depth`) 1))
      (`self.SpawnActorAtIndex` "/Game/Team/Woogle/Building/BP_SliceableConfDesk.BP_SliceableConfDesk_C" (- _output_get (`self.Depth`) -1))
      (`self.SpawnActorAtIndex` "/Game/Team/Woogle/Building/BP_SliceableCEODesk.BP_SliceableCEODesk_C" (- (`local.centerIndex`) 1) (struct :`Yaw` 180.0))
      (`self.SpawnActorAtIndex` "/Game/Team/Woogle/Building/BP_CEOBack.BP_CEOBack_C" (+ (`local.centerIndex`) -2) (struct :`Yaw` 180.0)))
    (:`then_1`
      (`self.SpawnActorAtIndex` "/Game/Team/Woogle/Building/BP_LobbyColumn.BP_LobbyColumn_C")
      (`self.SpawnActorAtIndex` "/Game/Team/Woogle/Building/BP_LobbyColumn.BP_LobbyColumn_C" (- (`self.Depth`) 1))
      (`self.SpawnActorAtIndex` "/Game/Team/Woogle/Building/BP_LobbyColumn.BP_LobbyColumn_C" _returnvalue)
      (`self.SpawnActorAtIndex` "/Game/Team/Woogle/Building/BP_LobbyColumn.BP_LobbyColumn_C" (- _returnvalue -1 (`self.Depth`))))
    (:`then_2`
      (`self.SpawnActorAtIndex` "/Game/Team/Woogle/Building/BP_Locker.BP_Locker_C" (+ (/ (`self.Depth`) 2) 1))
      (`self.SpawnActorAtIndex` "/Game/Team/Woogle/Building/BP_Locker.BP_Locker_C" (+ (/ (`self.Depth`) 2) -1))
      (`self.SpawnActorAtIndex` "/Game/Team/Woogle/Building/BP_Locker.BP_Locker_C" (- (* (`self.Depth`) (`self.Width`)) (/ (`self.Depth`) 2) 2) (struct :`Yaw` 180.0))
      (`self.SpawnActorAtIndex` "/Game/Team/Woogle/Building/BP_Locker.BP_Locker_C" (- (* (`self.Depth`) (`self.Width`)) (/ (`self.Depth`) 2)) (struct :`Yaw` 180.0)))
    (:`then_3`
      (`self.SpawnActorAtIndex` "/Game/Team/Woogle/Building/BP_WallShelf.BP_WallShelf_C" (/ (`self.Depth`) 2))
      (`self.SpawnActorAtIndex` "/Game/Team/Woogle/Building/BP_WallShelf.BP_WallShelf_C" (- (* (`self.Depth`) (`self.Width`)) (/ (`self.Depth`) 2) 1) (struct :`Yaw` 180.0)))))

(fn `UserConstructionScript`
  (locals (NewWallSacle :type "Vector Structure" :default (0.0 0.0 0.0)) (doorIndex :type Integer :default 0))
  (`parent.UserConstructionScript`))