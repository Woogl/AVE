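; BP_Interior04 is a procedural building interior variant that adds a dividing wall with a single doorway gap.
; The construction script runs the parent's, gives WallInstance a random material, and scales segments from mesh bounds to fit UnitSize.
; It picks a random line across the width and adds rotated wall instances along the depth, skipping one random index for the door.
; Relocation, prop and enemy spawning functions just call the parent.
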(fn `RelocateComp`
  (params (Comp :type "SceneComponent Object Reference"))
  (`parent.RelocateComp` Comp))

(fn `SpawnRandomEnemy`
  (`parent.SpawnRandomEnemy`))

(fn `SpawnRandomProp`
  (`parent.SpawnRandomProp`))

(fn `UserConstructionScript`
  (locals (NewWallSacle :type "Vector Structure" :default (0.0 0.0 0.0)) (doorIndex :type Integer :default 0))
  (bind (_unitsize_x _unitsize_y) (`KismetMathLibrary.BreakVector` (`self.UnitSize`)))
  (bind _unitsize_x_2 (`KismetMathLibrary.BreakVector` (`self.UnitSize`)))
  (bind (_unitsize_x_3 _unitsize_y_2 _unitsize_z) (`KismetMathLibrary.BreakVector` (`self.UnitSize`)))
  (bind (_min _max) (`StaticMeshComponent.GetLocalBounds` (`self.WallInstance`)))
  (bind _returnvalue (`KismetMathLibrary.FMax` (.x _max) (.y _max)))
  (`parent.UserConstructionScript`)
  ;[0 0 0] Vertical Wall
  (set `local.NewWallSacle` (`KismetMathLibrary.MakeVector` (/ _unitsize_x_3 _returnvalue) (/ _unitsize_y_2 _returnvalue) (/ _unitsize_z (.z _max))))
  (`PrimitiveComponent.SetMaterial` (`self.WallInstance`) 0 (`KismetArrayLibrary.Array_Random` (`self.RandomMaterials`)))
  (bind _output_get (set `self.WallLoc` (* _unitsize_x_2 (- (`KismetMathLibrary.RandomIntegerInRange` 1 (- (`self.Width`) 1)) (/ (`self.Width`) 2)))))
  (bind _output_get_2 (set `local.doorIndex` (`KismetMathLibrary.RandomIntegerInRange` 0 (- (`self.Depth`) 1))))
  (for _index (range (`self.Depth`))
    (if (not (== _index _output_get_2))
      (`InstancedStaticMeshComponent.AddInstance` (`self.WallInstance`) (`KismetMathLibrary.MakeTransform` (`KismetMathLibrary.MakeVector` _output_get (* _index _unitsize_y)) (struct :`Yaw` 90.0) (`local.NewWallSacle`)) false))))