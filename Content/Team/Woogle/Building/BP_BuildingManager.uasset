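; Manager actor that procedurally assembles a multi-floor building on BeginPlay from Width, Depth, Height and UnitSize.
; It spawns exterior, lobby, randomly chosen Interior03/04 middle floors, top-floor CEO room, cardkey front door, rooftop and elevator, stacking floors by UnitSize.Z.
; Spawned actors are tracked in BuildingElements for destroying or remaking; most floor actors receive a manager reference.
; OnPlayBossBattle replaces the building with only a rooftop and elevator at fixed heights.
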(event `self.ReceiveBeginPlay`
  (`self.MakeBuilding`))

(event `MakeBuilding`
  (`|ExecutionSequence`
    (:`then_0`
      (`self.SpawnExterior`))
    (:`then_1`
      (`self.SpawnLobby` 1))
    (:`then_2`
      (`self.SpawnInterior` 2)
      (for _index (range 3 (`self.Height`))
        (`self.SpawnInterior` _index true)))
    (:`then_3`
      (`self.SpawnCEORoom` (`self.Height`)))
    (:`then_4`
      (`self.SpawnFrontDoor`))
    (:`then_5`
      (`self.SpawnRoofTop`)
      (`self.SpawnElevator`))))

(event `DestroyBuilding`
  (bind _buildingelements (`self.BuildingElements`))
  (for _array_element _buildingelements
    (`/Engine/EditorBlueprintResources/StandardMacros.IsValid` _array_element
      (:`Is Valid`
        (`self.K2_DestroyActor` _array_element))))
  (`KismetArrayLibrary.Array_RemoveItem` _buildingelements))

(event `RemakeBuilding`
  (`self.DestroyBuilding`)
  (`self.MakeBuilding`))

(event `OnPlayBossBattle`
  (bind _returnvalue (`self.GetTransform`))
  (bind (_unitsize_x _unitsize_y _unitsize_z) (`KismetMathLibrary.BreakVector` (`self.UnitSize`)))
  (`self.DestroyBuilding`)
  ;[1 1 1] RoofTop, Elevator 4층 고정 소환
  (bind _returnvalue_2 (`|SpawnActorFromClass` "/Game/Team/Woogle/Building/BP_RoofTop.BP_RoofTop_C" (`KismetMathLibrary.MakeTransform` (`KismetMathLibrary.MakeVector` (.x (.location _returnvalue)) (.y (.location _returnvalue)) (+ (.z (.location _returnvalue)) (* _unitsize_z 4.0))) (.rotation _returnvalue) (.scale _returnvalue)) "AlwaysSpawn" "OverrideRootScale" null (`self.Width`) (`self.Depth`) (`self.Height`) (`self.UnitSize`) false null))
  (`KismetArrayLibrary.Array_Add` (`self.BuildingElements`) _returnvalue_2)
  (set `/Game/Team/Woogle/Building/BP_InteriorBase.BuildingManagerRef` self _returnvalue_2)
  (bind _returnvalue_3 (`self.SpawnElevator`))
  (`self.K2_AddActorLocalOffset` _returnvalue_3 (0.0 0.0 2400.0) false false))

(fn `SpawnCEORoom`
  (params (CurHeight :type Integer))
  (bind _returnvalue (`self.GetTransform`))
  (bind (_unitsize_x _unitsize_y _unitsize_z) (`KismetMathLibrary.BreakVector` (`self.UnitSize`)))
  (bind _returnvalue_2 (`|SpawnActorFromClass` "/Game/Team/Woogle/Building/BP_CEORoom.BP_CEORoom_C" (`KismetMathLibrary.MakeTransform` (`KismetMathLibrary.MakeVector` (.x (.location _returnvalue)) (.y (.location _returnvalue)) (+ (.z (.location _returnvalue)) (* _unitsize_z (- CurHeight 1)))) (.rotation _returnvalue) (.scale _returnvalue)) "AlwaysSpawn" "OverrideRootScale" null (`self.Width`) (`self.Depth`) CurHeight (`self.UnitSize`) true null))
  (`KismetArrayLibrary.Array_Add` (`self.BuildingElements`) _returnvalue_2))

(fn `SpawnElevator`
  (returns (ReturnValue :type "/Game/Team/Woogle/Building/BP_Elevator Object Reference"))
  (bind (_returnvalue_x _returnvalue_y _returnvalue_z) (`KismetMathLibrary.BreakVector` (`self.K2_GetActorLocation`)))
  (bind (_unitsize_x _unitsize_y) (`KismetMathLibrary.BreakVector` (`self.UnitSize`)))
  (bind (_unitsize_x_2 _unitsize_y_2) (`KismetMathLibrary.BreakVector` (`self.UnitSize`)))
  (bind _returnvalue (`|SpawnActorFromClass` "/Game/Team/Woogle/Building/BP_Elevator.BP_Elevator_C" (`KismetMathLibrary.MakeTransform` (`KismetMathLibrary.MakeVector` (+ _returnvalue_x (`KismetMathLibrary.SelectFloat` (* _unitsize_x_2 0.5) 0.0 (== (mod (`self.Width`) 2) 0))) (+ _returnvalue_y (* _unitsize_y_2 (`self.Depth`)) (* _unitsize_y 0.5)) _returnvalue_z)) "AlwaysSpawn" "OverrideRootScale" null (`self.UnitSize`) null))
  (`KismetArrayLibrary.Array_Add` (`self.BuildingElements`) _returnvalue)
  (return _returnvalue))

(fn `SpawnExterior`
  (bind _returnvalue (`|SpawnActorFromClass` "/Game/Team/Woogle/Building/BP_BuildingExterior.BP_BuildingExterior_C" (`self.GetTransform`) "AlwaysSpawn" "OverrideRootScale" null (`self.Width`) (`self.Depth`) (`self.Height`) (`self.UnitSize`) null))
  (`KismetArrayLibrary.Array_Add` (`self.BuildingElements`) _returnvalue))

(fn `SpawnFrontDoor`
  (bind (_returnvalue_location _returnvalue_rotation _returnvalue_scale) (`KismetMathLibrary.BreakTransform` (`self.GetTransform`)))
  (bind _unitsize_x (`KismetMathLibrary.BreakVector` (`self.UnitSize`)))
  (bind _returnvalue (`|SpawnActorFromClass` "/Game/Team/Woogle/Building/BP_CardkeyDoor.BP_CardkeyDoor_C" (`KismetMathLibrary.MakeTransform` (`KismetMathLibrary.MakeVector` (+ (.x _returnvalue_location) (`KismetMathLibrary.SelectFloat` (* _unitsize_x 0.5) 0.0 (== (mod (`self.Width`) 2) 0))) (.y _returnvalue_location) (.z _returnvalue_location)) (`KismetMathLibrary.MakeRotator` (.roll _returnvalue_rotation) (.pitch _returnvalue_rotation) (+ (.yaw _returnvalue_rotation) 90.0)) _returnvalue_scale) "AlwaysSpawn" "OverrideRootScale" null (`self.UnitSize`) null))
  (`KismetArrayLibrary.Array_Add` (`self.BuildingElements`) _returnvalue))

(fn `SpawnInterior`
  (params (CurHeight :type Integer) (bRandomUnderLighit :type Boolean))
  (bind _returnvalue (`self.GetTransform`))
  (bind (_unitsize_x _unitsize_y _unitsize_z) (`KismetMathLibrary.BreakVector` (`self.UnitSize`)))
  (bind _returnvalue_2 (`KismetMathLibrary.MakeTransform` (`KismetMathLibrary.MakeVector` (.x (.location _returnvalue)) (.y (.location _returnvalue)) (+ (.z (.location _returnvalue)) (* _unitsize_z (- CurHeight 1)))) (.rotation _returnvalue) (.scale _returnvalue)))
  (if (`KismetMathLibrary.RandomBool`)
    (bind _returnvalue_3 (`|SpawnActorFromClass` "/Game/Team/Woogle/Building/BP_Interior03.BP_Interior03_C" _returnvalue_2 "AlwaysSpawn" "OverrideRootScale" null (`self.Width`) (`self.Depth`) CurHeight (`self.UnitSize`) bRandomUnderLighit null))
    (`KismetArrayLibrary.Array_Add` (`self.BuildingElements`) _returnvalue_3)
    (set `/Game/Team/Woogle/Building/BP_InteriorBase.BuildingManagerRef` self _returnvalue_3)
    (else
      (bind _returnvalue_4 (`|SpawnActorFromClass` "/Game/Team/Woogle/Building/BP_Interior04.BP_Interior04_C" _returnvalue_2 "AlwaysSpawn" "OverrideRootScale" null (`self.Width`) (`self.Depth`) CurHeight (`self.UnitSize`) bRandomUnderLighit null))
      (`KismetArrayLibrary.Array_Add` (`self.BuildingElements`) _returnvalue_4)
      (set `/Game/Team/Woogle/Building/BP_InteriorBase.BuildingManagerRef` self _returnvalue_4))))

(fn `SpawnLobby`
  (params (CurHeight :type Integer))
  (bind _returnvalue (`|SpawnActorFromClass` "/Game/Team/Woogle/Building/BP_Lobby.BP_Lobby_C" (`self.GetTransform`) "AlwaysSpawn" "OverrideRootScale" null (`self.Width`) (`self.Depth`) CurHeight (`self.UnitSize`) false null))
  (`KismetArrayLibrary.Array_Add` (`self.BuildingElements`) _returnvalue)
  (set `/Game/Team/Woogle/Building/BP_InteriorBase.BuildingManagerRef` self _returnvalue))

(fn `SpawnRoofTop`
  (returns (ReturnValue :type "/Game/Team/Woogle/Building/BP_RoofTop Object Reference"))
  (bind _returnvalue (`self.GetTransform`))
  (bind (_unitsize_x _unitsize_y _unitsize_z) (`KismetMathLibrary.BreakVector` (`self.UnitSize`)))
  (bind _returnvalue_2 (`|SpawnActorFromClass` "/Game/Team/Woogle/Building/BP_RoofTop.BP_RoofTop_C" (`KismetMathLibrary.MakeTransform` (`KismetMathLibrary.MakeVector` (.x (.location _returnvalue)) (.y (.location _returnvalue)) (+ (.z (.location _returnvalue)) (* _unitsize_z (`self.Height`)))) (.rotation _returnvalue) (.scale _returnvalue)) "AlwaysSpawn" "OverrideRootScale" null (`self.Width`) (`self.Depth`) (`self.Height`) (`self.UnitSize`) false null))
  (`KismetArrayLibrary.Array_Add` (`self.BuildingElements`) _returnvalue_2)
  (set `/Game/Team/Woogle/Building/BP_InteriorBase.BuildingManagerRef` self _returnvalue_2)
  (return _returnvalue_2))

(fn `UserConstructionScript`)