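; Elevator actor that carries play between stages, tracking the current floor and whether the stage is won.
; StageWin dings and opens the sliding timeline-driven doors, while an overlap trigger closes them during an unwon stage and re-arms a DoOnce.
; A second trigger fires that DoOnce to close the doors and lerp the car up one unit height, then StageStart reopens them.
; Tab forces StageWin for debugging.
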(event `OpenDoor`
  (bind (_direction _position) (`Timeline|TL_OpenLDoor` :!via `PlayFromStart`)
    (:`Update`
      (`|ExecutionSequence`
        (:`then_0`
          (`SceneComponent.K2_SetRelativeLocation` (`self.LeftDoor`) (`KismetMathLibrary.MakeVector` (+ _position -113.0) 290.0 15.0) false false))
        (:`then_1`
          (`SceneComponent.K2_SetRelativeLocation` (`self.RightDoor`) (`KismetMathLibrary.MakeVector` (+ (* _position -1.0) 113.0) 290.0 15.0) false false))))
    (:`Finished`
      (set `self.bIsClosed` false))))

(event `self.ReceiveBeginPlay`
  ;[1 1 1] debug
  (`KismetSystemLibrary.Delay` 0.2)
  (`self.EnableInput` (`GameplayStatics.GetPlayerController` 0)))

(event `CloseDoor`
  (bind (_direction _position) (`Timeline|Timeline_0` :!via `ReverseFromEnd`)
    (:`Update`
      (`|ExecutionSequence`
        (:`then_0`
          (`SceneComponent.K2_SetRelativeLocation` (`self.LeftDoor`) (`KismetMathLibrary.MakeVector` (+ _position -113.0) 290.0 15.0) false false))
        (:`then_1`
          (`SceneComponent.K2_SetRelativeLocation` (`self.RightDoor`) (`KismetMathLibrary.MakeVector` (+ (* _position -1.0) 113.0) 290.0 15.0) false false))))
    (:`Finished`
      (set `self.bIsClosed` true))))

(event `Key|Tab`
  (params (Key :type "Key Structure"))
  ;[1 1 1] debug
  (:`Pressed`
    (`self.StageWin`)))

(event `self.SwitchCloseDoor.OnComponentBeginOverlap`
  (params (OverlappedComponent :type "PrimitiveComponent Object Reference") (OtherActor :type "Actor Object Reference") (OtherComp :type "PrimitiveComponent Object Reference") (OtherBodyIndex :type Integer) (bFromSweep :type Boolean) (SweepResult :type "HitResult Structure (by ref)"))
  (if (and (not (`self.bIsClosed`)) (not (`self.bIsWon`)))
    (`self.CloseDoor`)
    (goto _label :!via `Reset`)))

(event `StageStart`
  (set `self.bIsWon` false)
  (`self.OpenDoor`)
  (`/Engine/EditorBlueprintResources/StandardMacros.IncrementInt` (`self.CurrentFloor`)))

(event `StageWin`
  (set `self.bIsWon` true)
  (`GameplayStatics.PlaySoundAtLocation` "/Game/Team/Woogle/Sounds/SW_ElevatorDing.SW_ElevatorDing" (`self.K2_GetActorLocation`) (struct) 1.0 1.0 0.0 null null null null)
  (`self.OpenDoor`))

(event `self.SwitchLiftElevator.OnComponentBeginOverlap`
  (params (OverlappedComponent :type "PrimitiveComponent Object Reference") (OtherActor :type "Actor Object Reference") (OtherComp :type "PrimitiveComponent Object Reference") (OtherBodyIndex :type Integer) (bFromSweep :type Boolean) (SweepResult :type "HitResult Structure (by ref)"))
  (`/Engine/EditorBlueprintResources/StandardMacros.DoOnce` false :!label _label
    (:`Completed`
      (`self.CloseDoor`)
      (`KismetSystemLibrary.Delay` 1.0)
      (`self.LiftElevator`))))

(event `LiftElevator`
  (bind (_unitsize_x _unitsize_y _unitsize_z) (`KismetMathLibrary.BreakVector` (`self.UnitSize`)))
  (bind _output_get (set `self.StartLoc` (`self.K2_GetActorLocation`)))
  (set `self.EndLoc` (+ _output_get (`KismetMathLibrary.MakeVector` 0.0 0.0 _unitsize_z)))
  (`GameplayStatics.PlaySoundAtLocation` "/Game/Team/Woogle/Sounds/engine_high-71367.engine_high-71367" (`self.K2_GetActorLocation`) (struct) 1.0 1.0 0.0 null null null null)
  (bind (_direction _alpha) (`Timeline|TL_Lift` :!via `PlayFromStart`)
    (:`Update`
      (`self.K2_SetActorLocation` (`KismetMathLibrary.VLerp` (`self.StartLoc`) (`self.EndLoc`) _alpha)))
    (:`Finished`
      (`self.StageStart`)
      (`GameplayStatics.PlaySoundAtLocation` "/Game/Team/Woogle/Sounds/SW_ElevatorDing.SW_ElevatorDing" (`self.K2_GetActorLocation`) (struct) 1.0 1.0 0.0 null null null null))))

(fn `UserConstructionScript`)