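; BP_WallShelf is a wall shelf prop that randomizes three books for visual variety.
; Its construction script calls ChangeBookState on each book component.
; That function picks a random material from the BookMat array, randomizes scale per axis, slides the book along local Y within a fixed range, and randomly leaves it upright or rolls it 90 degrees.
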(fn `Change Book State`
  (params (BookToChange :type "PrimitiveComponent Object Reference"))
  (bind _returnvalue (`KismetMathLibrary.RandomFloatInRange` 0.6 0.9))
  (bind (_relativelocation_x _relativelocation_y _relativelocation_z) (`KismetMathLibrary.BreakVector` (`SceneComponent.RelativeLocation` BookToChange)))
  (`PrimitiveComponent.SetMaterial` BookToChange 0 (`KismetArrayLibrary.Array_Random` (`self.BookMat`)))
  (`SceneComponent.SetRelativeScale3D` BookToChange (`KismetMathLibrary.MakeVector` _returnvalue _returnvalue _returnvalue))
  (`SceneComponent.K2_SetRelativeLocationAndRotation` BookToChange (`KismetMathLibrary.MakeVector` _relativelocation_x (`KismetMathLibrary.RandomFloatInRange` -200.0 0.0) _relativelocation_z) (`KismetMathLibrary.MakeRotator` (`KismetMathLibrary.SelectFloat` 0.0 -90.0 (`KismetMathLibrary.RandomBool`))) false false))

(fn `UserConstructionScript`
  (`self.Change Book State` (`self.Book1`))
  (`self.Change Book State` (`self.Book2`))
  (`self.Change Book State` (`self.Book3`)))