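; Procedural building exterior that assembles a randomized box shell of wall meshes in its construction script, sized by Width, Depth, Height and UnitSize.
; Each RandomWalls mesh becomes an instanced static mesh component with a bounds-derived scale to fit the unit grid.
; Four sides are filled with random picks, leaving a front ground-floor opening and an empty middle back column.
; If NeonSignMesh is valid, randomly placed, scaled signs are added per RandomSignMats material.
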(fn `UserConstructionScript`
  (bind _width (`self.Width`))
  (bind (_unitsize_x _unitsize_y _unitsize_z) (`KismetMathLibrary.BreakVector` (`self.UnitSize`)))
  (bind _wallstoattach (`self.WallsToAttach`))
  (bind _unitsize_x_2 (`KismetMathLibrary.BreakVector` (`self.UnitSize`)))
  (bind (_unitsize_x_3 _unitsize_y_2 _unitsize_z_2) (`KismetMathLibrary.BreakVector` (`self.UnitSize`)))
  (bind _wallstoattach_2 (`self.WallsToAttach`))
  (bind _unitsize_x_4 (`KismetMathLibrary.BreakVector` (`self.UnitSize`)))
  (bind (_unitsize_x_5 _unitsize_y_3) (`KismetMathLibrary.BreakVector` (`self.UnitSize`)))
  (bind (_unitsize_x_6 _unitsize_y_4 _unitsize_z_3) (`KismetMathLibrary.BreakVector` (`self.UnitSize`)))
  (bind _wallstoattach_3 (`self.WallsToAttach`))
  (bind (_unitsize_x_7 _unitsize_y_5) (`KismetMathLibrary.BreakVector` (`self.UnitSize`)))
  (bind (_unitsize_x_8 _unitsize_y_6 _unitsize_z_4) (`KismetMathLibrary.BreakVector` (`self.UnitSize`)))
  (bind (_unitsize_x_9 _unitsize_y_7 _unitsize_z_5) (`KismetMathLibrary.BreakVector` (`self.UnitSize`)))
  (bind (_unitsize_x_10 _unitsize_y_8) (`KismetMathLibrary.BreakVector` (`self.UnitSize`)))
  (bind (_unitsize_x_11 _unitsize_y_9 _unitsize_z_6) (`KismetMathLibrary.BreakVector` (`self.UnitSize`)))
  (bind _wallstoattach_4 (`self.WallsToAttach`))
  (bind _returnvalue (`KismetMathLibrary.RandomIntegerInRange` 0 (- (`KismetArrayLibrary.Array_Length` _wallstoattach) 1)))
  (bind _returnvalue_2 (`KismetMathLibrary.RandomIntegerInRange` 0 (- (`KismetArrayLibrary.Array_Length` _wallstoattach_2) 1)))
  (bind _returnvalue_3 (`KismetMathLibrary.RandomIntegerInRange` 0 (- (`KismetArrayLibrary.Array_Length` _wallstoattach_3) 1)))
  (bind _returnvalue_4 (`KismetMathLibrary.RandomIntegerInRange` 0 (- (`KismetArrayLibrary.Array_Length` _wallstoattach_4) 1)))
  (bind (_output_x _output_y _output_z) (`KismetMathLibrary.BreakVector` (`|GetArrayItem` (`self.NewWallsScales`) _returnvalue_3)))
  (bind (_output_x_2 _output_y_2 _output_z_2) (`KismetMathLibrary.BreakVector` (`|GetArrayItem` (`self.NewWallsScales`) _returnvalue_4)))
  (`|ExecutionSequence`
    (:`then_0`
      ;[0 0 0] Instanced Static Mesh Comp 붙이기
      (for _array_element (`self.RandomWalls`)
        (bind _returnvalue_5 (`AddComponent|NODE_AddInstancedStaticMeshComponent-1`))
        (`SceneComponent.K2_SetRelativeLocation` _returnvalue_5 (`KismetMathLibrary.MakeVector` (/ (* _unitsize_x_4 (`self.Width`)) -2)) false false)
        (`KismetArrayLibrary.Array_Add` (`self.WallsToAttach`) _returnvalue_5)
        (`StaticMeshComponent.SetStaticMesh` _returnvalue_5 _array_element)
        (bind (_min _max) (`StaticMeshComponent.GetLocalBounds` _returnvalue_5))
        (bind _returnvalue_6 (`KismetMathLibrary.FMax` (.x _max) (.y _max)))
        (`KismetArrayLibrary.Array_Add` (`self.NewWallsScales`) (`KismetMathLibrary.MakeVector` (/ _unitsize_x_11 _returnvalue_6) (/ _unitsize_y_9 _returnvalue_6) (/ _unitsize_z_6 (.z _max))))))
    (:`then_1`
      ;[0 0 0] Front Wall
      (for _index (range (`self.Height`))
        (for _index_2 (range (`self.Width`))
          (if (not (and (== _index 0) (== _index_2 (/ (`self.Width`) 2))))
            (`InstancedStaticMeshComponent.AddInstance` (`|GetArrayItem` _wallstoattach _returnvalue) (`KismetMathLibrary.MakeTransform` (`KismetMathLibrary.MakeVector` (* _unitsize_x_2 _index_2) 0.0 (* _unitsize_z_2 _index)) (struct) (`|GetArrayItem` (`self.NewWallsScales`) _returnvalue)) false)))))
    (:`then_2`
      ;[0 0 0] Back Wall
      (for _index_3 (range (`self.Height`))
        (for _index_4 (range (`self.Width`))
          (if (not (== _index_4 (/ (`self.Width`) 2)))
            (`InstancedStaticMeshComponent.AddInstance` (`|GetArrayItem` _wallstoattach_2 _returnvalue_2) (`KismetMathLibrary.MakeTransform` (`KismetMathLibrary.MakeVector` (* _unitsize_x_5 (+ _index_4 1)) (* _unitsize_y_3 (`self.Depth`)) (* _unitsize_z_3 _index_3)) (struct :`Yaw` 180.0) (`|GetArrayItem` (`self.NewWallsScales`) _returnvalue_2)) false)))))
    (:`then_3`
      ;[0 0 0] Left Wall
      (for _index_5 (range (`self.Height`))
        (for _index_6 (range (`self.Depth`))
          (`InstancedStaticMeshComponent.AddInstance` (`|GetArrayItem` _wallstoattach_3 _returnvalue_3) (`KismetMathLibrary.MakeTransform` (`KismetMathLibrary.MakeVector` (* _unitsize_x_10 (`self.Width`)) (* _unitsize_y_8 (+ _index_6 1)) (* _unitsize_z_4 _index_5)) (struct :`Yaw` -90.0) (`KismetMathLibrary.MakeVector` _output_y _output_x _output_z)) false))))
    (:`then_4`
      ;[0 0 0] Right Wall
      (for _index_7 (range (`self.Height`))
        (for _index_8 (range (`self.Depth`))
          (`InstancedStaticMeshComponent.AddInstance` (`|GetArrayItem` _wallstoattach_4 _returnvalue_4) (`KismetMathLibrary.MakeTransform` (`KismetMathLibrary.MakeVector` 0.0 (* _unitsize_y_5 _index_8) (* _unitsize_z _index_7)) (struct :`Yaw` 90.0) (`KismetMathLibrary.MakeVector` _output_y_2 _output_x_2 _output_z_2)) false))))
    (:`then_5`
      ;[0 0 0] Sign
      (`/Engine/EditorBlueprintResources/StandardMacros.IsValid` (`self.NeonSignMesh`)
        (:`Is Valid`
          (for _index_9 (range (`KismetArrayLibrary.Array_Length` (`self.RandomSignMats`)))
            (bind _returnvalue_7 (`AddComponent|NODE_AddStaticMeshComponent-1` :`RelativeTransform` (`KismetMathLibrary.MakeTransform` (`KismetMathLibrary.MakeVector` (* _unitsize_x_9 (`KismetMathLibrary.RandomFloatInRange` (+ (* _width -0.5) 1.5) (+ (* _width 0.5) -1.5))) -50.0 (* _unitsize_z_5 (`KismetMathLibrary.RandomFloatInRange` 2.0 (`KismetMathLibrary.Conv_IntToDouble` (- (`self.Height`) 1))))) (struct :`Yaw` 180.0 :`Roll` 90.0) (`KismetMathLibrary.MakeVector` (`KismetMathLibrary.RandomFloatInRange` 4.0 14.0) (`KismetMathLibrary.RandomFloatInRange` 4.0 14.0) 4.0))))
            (`PrimitiveComponent.SetMaterial` _returnvalue_7 0 (`|GetArrayItem` (`self.RandomSignMats`) _index_9))))))))