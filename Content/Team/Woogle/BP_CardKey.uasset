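; BP_CardKey is a card key pickup that signals its target door when obtained.
; An outer-named HighlightSphere toggles custom depth on the mesh as overlaps begin and end, for highlighting.
; Overlapping ObtainSphere hides the mesh, sends StageCleared to TargetDoor and a pickup message to the overlapping actor.
; It then sets a short lifespan and clears that message in the same execution chain, with no delay.
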(event `self.HighlightSphere.OnComponentBeginOverlap`
  (params (OverlappedComponent :type "PrimitiveComponent Object Reference") (OtherActor :type "Actor Object Reference") (OtherComp :type "PrimitiveComponent Object Reference") (OtherBodyIndex :type Integer) (bFromSweep :type Boolean) (SweepResult :type "HitResult Structure (by ref)"))
  (`PrimitiveComponent.SetRenderCustomDepth` (`self.StaticMesh`) true))

(event `self.ObtainSphere.OnComponentBeginOverlap`
  (params (OverlappedComponent :type "PrimitiveComponent Object Reference") (OtherActor :type "Actor Object Reference") (OtherComp :type "PrimitiveComponent Object Reference") (OtherBodyIndex :type Integer) (bFromSweep :type Boolean) (SweepResult :type "HitResult Structure (by ref)"))
  (`SceneComponent.SetVisibility` (`self.StaticMesh`) false false)
  (message `/Game/Team/Woogle/BPI_CardKeyDoor.StageCleared` (`self.TargetDoor`))
  (message `/Game/Blueprints/BPI_Player.ShowDirectiveMessage` OtherActor "You got the card key.")
  (`self.SetLifeSpan` 4.0)
  (message `/Game/Blueprints/BPI_Player.ShowDirectiveMessage` OtherActor ""))

(event `self.HighlightSphere.OnComponentEndOverlap`
  (params (OverlappedComponent :type "PrimitiveComponent Object Reference") (OtherActor :type "Actor Object Reference") (OtherComp :type "PrimitiveComponent Object Reference") (OtherBodyIndex :type Integer))
  (`PrimitiveComponent.SetRenderCustomDepth` (`self.StaticMesh`) false))

(fn `UserConstructionScript`)