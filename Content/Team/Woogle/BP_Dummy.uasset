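; BP_Dummy is a hit-reaction dummy that responds to point damage with animations.
; On each hit it sets its yaw with a look-at rotation from its location, passing ShotFromDirection as the target.
; It reads the damage type from the hit result's HitItem field, cast to EDamageType, and prints it.
; That type selects a standard, knock back, knock down or knock up montage.
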(event `self.ReceivePointDamage`
  (params (Damage :type "Float (single-precision)") (DamageType :type "DamageType Object Reference") (HitLocation :type "Vector Structure") (HitNormal :type "Vector Structure") (HitComponent :type "PrimitiveComponent Object Reference") (BoneName :type Name) (ShotFromDirection :type "Vector Structure") (InstigatedBy :type "Controller Object Reference") (DamageCauser :type "Actor Object Reference") (HitInfo :type "HitResult Structure (by ref)"))
  (bind (_returnvalue_roll _returnvalue_pitch) (`KismetMathLibrary.BreakRotator` (`self.K2_GetActorRotation`)))
  (bind (_returnvalue_roll_2 _returnvalue_pitch_2 _returnvalue_yaw) (`KismetMathLibrary.BreakRotator` (`KismetMathLibrary.FindLookAtRotation` (`self.K2_GetActorLocation`) ShotFromDirection)))
  (bind _returnvalue (cast `EDamageType` (`KismetMathLibrary.Conv_IntToByte` (`.HitItem` (`GameplayStatics.BreakHitResult` HitInfo)))))
  (`self.K2_SetActorRotation` (`KismetMathLibrary.MakeRotator` _returnvalue_roll _returnvalue_pitch _returnvalue_yaw))
  (`KismetSystemLibrary.PrintString` (`|GetEnumeratorNameAsString` _returnvalue))
  (switch `EDamageType` _returnvalue
    (:`EDT_Standard`
      (`self.PlayAnimMontage` "/Game/Team/Woogle/Animations/Hit/HitStandard.HitStandard"))
    (:`EDT_KnockBack`
      (`self.PlayAnimMontage` "/Game/Team/Woogle/Animations/Hit/KnockBack.KnockBack"))
    (:`EDT_KnockDown`
      (`self.PlayAnimMontage` "/Game/Team/Woogle/Animations/Hit/Anim_down_01_Montage.Anim_down_01_Montage"))
    (:`EDT_KnockUp`
      (`self.PlayAnimMontage` "/Game/Team/Woogle/Animations/Hit/GhostSamurai_APose_Hit_Up_Inplace_Montage.GhostSamurai_APose_Hit_Up_Inplace_Montage"))))

(fn `UserConstructionScript`)