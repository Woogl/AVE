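; BP_DamageTester is a test actor that applies a fixed point of damage with a selectable reaction type to actors overlapping its box.
; Box overlap calls ApplyPointDamage, passing the tester's location as HitFromDirection.
; The DamageType enum travels as an integer in the HitResult's HitItem field rather than through a damage type class.
; The construction script labels the TextRender with the selected type.
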(event `self.Box.OnComponentBeginOverlap`
  (params (OverlappedComponent :type "PrimitiveComponent Object Reference") (OtherActor :type "Actor Object Reference") (OtherComp :type "PrimitiveComponent Object Reference") (OtherBodyIndex :type Integer) (bFromSweep :type Boolean) (SweepResult :type "HitResult Structure (by ref)"))
  (`GameplayStatics.ApplyPointDamage` OtherActor 10.0 (`self.K2_GetActorLocation`) (`GameplayStatics.MakeHitResult` false false 0.0 0.0 (0.0 0.0 0.0) (0.0 0.0 0.0) (0.0 0.0 1.0) (0.0 0.0 1.0) null null null "None" "None" (`KismetMathLibrary.Conv_ByteToInt` (`self.DamageType`))) null self))

(fn `UserConstructionScript`
  (bind _textrender (`self.TextRender`))
  (switch `EDamageType` (`self.DamageType`)
    (:`EDT_Standard`
      (`TextRenderComponent.K2_SetText` _textrender "Standard"))
    (:`EDT_KnockBack`
      (`TextRenderComponent.K2_SetText` _textrender "Knock \nBack"))
    (:`EDT_KnockDown`
      (`TextRenderComponent.K2_SetText` _textrender "Knock \nDown"))
    (:`EDT_KnockUp`
      (`TextRenderComponent.K2_SetText` _textrender "Knock \nUp"))
    (:`EDT_NoReaction`
      (`TextRenderComponent.K2_SetText` _textrender "No \nReaction"))))