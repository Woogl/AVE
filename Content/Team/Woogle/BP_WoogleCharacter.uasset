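; Player-style character Blueprint that implements landing recovery, finisher takedowns and afterimage effects, with some events declared in C++.
; Landing disables movement briefly, holding longer if a montage is playing.
; MotionMorph sets a motion-warp target just short of the enemy, facing it, then calls FinishEnemy and notifies Dummy targets.
; SpawnGhostTrail spawns an afterimage at the mesh transform, and an anim notify event sets rotation interp speed.
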(event `self.OnLanded`
  (params (Hit :type "HitResult Structure (by ref)"))
  ;[1 1 1] 착지
  (`CharacterMovementComponent.SetMovementMode` (`self.CharacterMovement`) "MOVE_None" 0)
  (if (`AnimInstance.IsAnyMontagePlaying` (`SkeletalMeshComponent.GetAnimInstance` (`self.Mesh`)))
    (`KismetSystemLibrary.Delay` 1.0)
    (else
      (`KismetSystemLibrary.Delay` 0.6)))
  (`CharacterMovementComponent.SetMovementMode` (`self.CharacterMovement`) "MOVE_Walking" 0))

(event `self.MotionMorph`
  (bind (_returnvalue_roll _returnvalue_pitch) (`KismetMathLibrary.BreakRotator` (`self.K2_GetActorRotation`)))
  (bind _returnvalue (`self.K2_GetActorLocation` (`self.EnemyTarget`)))
  (bind (_returnvalue_roll_2 _returnvalue_pitch_2 _returnvalue_yaw) (`KismetMathLibrary.BreakRotator` (`KismetMathLibrary.FindLookAtRotation` (`self.K2_GetActorLocation`) (`self.K2_GetActorLocation` (`self.EnemyTarget`)))))
  ;[1 1 1] 모션 워핑
  (`MotionWarpingComponent.AddOrUpdateWarpTargetFromLocationAndRotation` (`self.MotionWarping`) "TakeDown01" (+ (* (`KismetMathLibrary.Normal` (- (`self.K2_GetActorLocation`) _returnvalue)) 80.0) _returnvalue) (`KismetMathLibrary.MakeRotator` _returnvalue_roll _returnvalue_pitch _returnvalue_yaw))
  (`self.FinishEnemy`)
  (bind _asdummy (cast `Dummy` (`self.EnemyTarget`)))
  (`Dummy.OnFinishered` _asdummy))

(event `self.SpawnGhostTrail`
  ;[1 1 1] 잔상
  (`|SpawnActorFromClass` "/Game/Team/Woogle/BP_GhostTrail.BP_GhostTrail_C" (`SceneComponent.K2_GetComponentToWorld` (`self.Mesh`)) "AlwaysSpawn" "OverrideRootScale" null self null))

(event `/Game/Blueprints/BPI_Player.SetRInterpSpeed`
  (params (RInterpSpeed :type "Float (double-precision)"))
  ;[1 1 1] Anim Notify
  (set `self.RInterpSpeed` RInterpSpeed))

(fn `UserConstructionScript`)