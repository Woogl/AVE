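; BP_Bullet is a projectile actor from the GunEnemy folder that flies straight until it touches the player.
; Tick moves it along its forward vector by Speed scaled by delta time, without sweep or a movement component.
; On overlap with BP_ThirdPersonCharacter it spawns the P_Hit emitter and destroys itself, applying no damage.
; Other overlaps are ignored, and the graph sets no lifetime.
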(event `self.ReceiveTick`
  (params (DeltaSeconds :type "Float (single-precision)"))
  ;[0 0 0] 총알 발사
  (`self.K2_SetActorLocation` (+ (`self.K2_GetActorLocation`) (* (* (`self.GetActorForwardVector`) (`self.Speed`)) DeltaSeconds))))

(event `self.ReceiveActorBeginOverlap`
  (params (OtherActor :type "Actor Object Reference"))
  ;[0 0 0] 감지되면 파괴
  (cast `/Game/ThirdPerson/Blueprints/BP_ThirdPersonCharacter` OtherActor)
  (`GameplayStatics.SpawnEmitterAtLocation` "/Game/MarketplaceAssets/Nodachi_Animset/demo/Particles/P_Hit.P_Hit" (`self.K2_GetActorLocation`))
  (`self.K2_DestroyActor`))

(fn `UserConstructionScript`)