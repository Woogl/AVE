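; Mun character Blueprint that handles melee combat reactions, landing recovery and finishers on top of C++ logic.
; Damage drains posture while blocking and health otherwise, while point damage plays parry, block or hit montages using a damage type encoded in HitItem.
; The C++-declared MotionMorph event sets a motion-warp target beside the enemy, triggers the finisher and notifies Dummy targets.
; Landing briefly disables movement, and an anim-notify event sets rotation interpolation speed.
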(event `self.OnLanded`
  (params (Hit :type "HitResult Structure (by ref)"))
  ;[1 1 1] 착지
  (`CharacterMovementComponent.SetMovementMode` (`self.CharacterMovement`) "MOVE_None" 0)
  (if (`AnimInstance.IsAnyMontagePlaying` (`SkeletalMeshComponent.GetAnimInstance` (`self.Mesh`)))
    (`KismetSystemLibrary.Delay` 1.0)
    (else
      (`KismetSystemLibrary.Delay` 0.6)))
  (`CharacterMovementComponent.SetMovementMode` (`self.CharacterMovement`) "MOVE_Walking" 0))

(event `self.ReceiveAnyDamage`
  (params (Damage :type "Float (single-precision)") (DamageType :type "DamageType Object Reference") (InstigatedBy :type "Controller Object Reference") (DamageCauser :type "Actor Object Reference"))
  (if (`self.bIsBlocking`)
    (bind _output_get (set `self.CurPosture` (- (`self.CurPosture`) Damage)))
    (`KismetSystemLibrary.PrintString` (`KismetStringLibrary.Concat_StrStr` "Posture: " (`KismetStringLibrary.Conv_DoubleToString` _output_get)))
    (else
      (bind _output_get_2 (set `self.CurHealth` (- (`self.CurHealth`) Damage)))
      (`KismetSystemLibrary.PrintString` (`KismetStringLibrary.Concat_StrStr` "Health: " (`KismetStringLibrary.Conv_DoubleToString` _output_get_2))))))

(event `self.MotionMorph`
  (bind (_returnvalue_roll _returnvalue_pitch) (`KismetMathLibrary.BreakRotator` (`self.K2_GetActorRotation`)))
  (bind _returnvalue (`self.K2_GetActorLocation` (`self.EnemyTarget`)))
  (bind (_returnvalue_roll_2 _returnvalue_pitch_2 _returnvalue_yaw) (`KismetMathLibrary.BreakRotator` (`KismetMathLibrary.FindLookAtRotation` (`self.K2_GetActorLocation`) (`self.K2_GetActorLocation` (`self.EnemyTarget`)))))
  ;[1 1 1] 모션 워핑
  (`MotionWarpingComponent.AddOrUpdateWarpTargetFromLocationAndRotation` (`self.MotionWarping`) "TakeDown01" (+ (* (`KismetMathLibrary.Normal` (- (`self.K2_GetActorLocation`) _returnvalue)) 80.0) _returnvalue) (`KismetMathLibrary.MakeRotator` _returnvalue_roll _returnvalue_pitch _returnvalue_yaw))
  (`self.FinishEnemy`)
  (bind _asdummy (cast `Dummy` (`self.EnemyTarget`)))
  (`Dummy.OnFinishered` _asdummy))

(event `self.ReceivePointDamage`
  (params (Damage :type "Float (single-precision)") (DamageType :type "DamageType Object Reference") (HitLocation :type "Vector Structure") (HitNormal :type "Vector Structure") (HitComponent :type "PrimitiveComponent Object Reference") (BoneName :type Name) (ShotFromDirection :type "Vector Structure") (InstigatedBy :type "Controller Object Reference") (DamageCauser :type "Actor Object Reference") (HitInfo :type "HitResult Structure (by ref)"))
  (bind _returnvalue (cast `EDamageType` (`KismetMathLibrary.Conv_IntToByte` (`.HitItem` (`GameplayStatics.BreakHitResult` HitInfo)))))
  (`KismetSystemLibrary.PrintString` (`|GetEnumeratorNameAsString` _returnvalue))
  (if (`self.bIsBlocking`)
    (if (`self.bIsParrying`)
      (switch `EDamageType` _returnvalue
        (:`EDT_Standard`
          _)
        (:`EDT_KnockBack`
          _)
        (:`EDT_KnockDown`
          _)
        (:`EDT_KnockUp`
          _))
      (`self.PlayAnimMontage` "/Game/Woogle/Animations/Hit/GhostSamurai_DefenseR_Parry01_Root_Montage.GhostSamurai_DefenseR_Parry01_Root_Montage")
      (else
        (switch `EDamageType` _returnvalue
          (:`EDT_Standard`
            _)
          (:`EDT_KnockBack`
            _)
          (:`EDT_KnockDown`
            _)
          (:`EDT_KnockUp`
            _))
        (`self.PlayAnimMontage` "/Game/Woogle/Animations/Hit/GhostSamurai_DefenseR_Hit01_Root_Montage.GhostSamurai_DefenseR_Hit01_Root_Montage")))
    (else
      (switch `EDamageType` _returnvalue
        (:`EDT_Standard`
          (`self.PlayAnimMontage` "/Game/Woogle/Animations/Hit/HitStandard.HitStandard"))
        (:`EDT_KnockBack`
          (`self.PlayAnimMontage` "/Game/Woogle/Animations/Hit/KnockBack.KnockBack"))
        (:`EDT_KnockDown`
          (`self.PlayAnimMontage` "/Game/Woogle/Animations/Hit/Anim_down_01_Montage.Anim_down_01_Montage"))
        (:`EDT_KnockUp`
          (`self.PlayAnimMontage` "/Game/Woogle/Animations/Hit/GhostSamurai_APose_Hit_Up_Inplace_Montage.GhostSamurai_APose_Hit_Up_Inplace_Montage"))))))

(event `/Game/Blueprints/BPI_Player.SetRInterpSpeed`
  (params (RInterpSpeed :type "Float (double-precision)"))
  ;[1 1 1] Anim Notify
  (set `self.RInterpSpeed` RInterpSpeed))

(fn `UserConstructionScript`)