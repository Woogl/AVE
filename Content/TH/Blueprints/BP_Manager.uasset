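; BP_Manager coordinates the BP_Swordman enemies as a group and tracks which remain.
; On BeginPlay it caches the player and all swordmen and adds the WBP_StateCounter widget to the viewport.
; StartAI, gated by a one-shot flag, runs BT_Manager on its own AI controller and writes AIState to each enemy's blackboard, skipping those in one particular state.
; EnemyDie removes an enemy from the list; its empty-list check triggers nothing.
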(event `self.ReceiveBeginPlay`
  (bind _returnvalue (`GameplayStatics.GetActorOfClass` "/Game/TH/Blueprints/BP_THPlayer.BP_THPlayer_C"))
  (set `self.PlayerActor` _returnvalue)
  (bind _outactors (`GameplayStatics.GetAllActorsOfClass` "/Game/TH/Blueprints/BP_Swordman.BP_Swordman_C"))
  (set `self.Enemies` _outactors)
  (bind _returnvalue_2 (`|CreateWidget` "/Game/TH/Blueprints/WBP_StateCounter.WBP_StateCounter_C"))
  (`UserWidget.AddToViewport` _returnvalue_2 0))

(fn `EnemyDie`
  (params (NewParam :type "/Game/TH/Blueprints/BP_Swordman Object Reference"))
  (bind _enemies (`self.Enemies`))
  (`KismetArrayLibrary.Array_RemoveItem` _enemies NewParam)
  (if (<= (`KismetArrayLibrary.Array_Length` _enemies) 0)
    _))

(fn `StartAI`
  (locals (AIState :type Name :default "AIState") (Enum :type Byte :default 1) (Player :type Name :default "PlayerActor"))
  (if (`self.On`)
    (`AIController.RunBehaviorTree` (`AIBlueprintHelperLibrary.GetAIController` self) "/Game/TH/Tree/Manager/BT_Manager.BT_Manager")
    (set `self.On` false)
    (for _array_element (`self.Enemies`)
      (bind _returnvalue (`AIBlueprintHelperLibrary.GetBlackboard` _array_element))
      (if (!= (`BlackboardComponent.GetValueAsEnum` _returnvalue (`local.AIState`)) 4)
        (`BlackboardComponent.SetValueAsEnum` _returnvalue (`local.AIState`) (`local.Enum`))))))

(fn `UserConstructionScript`)