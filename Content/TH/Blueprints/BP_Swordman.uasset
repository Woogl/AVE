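; Swordsman enemy with health and posture, linked to BP_Manager and driven by an AI controller blackboard.
; Damage lowers both stats, sets the AI state, reports a damage event and calls StartAI on the manager.
; A looping timer regenerates posture, and depleting it flags Broken on the blackboard.
; Zero health plays a death montage, while manager notification, ragdoll and destroy logic sit unconnected.
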(event `self.ReceiveBeginPlay`
  (bind _returnvalue (`GameplayStatics.GetActorOfClass` "/Game/TH/Blueprints/BP_Manager.BP_Manager_C"))
  (set `self.AIManager` _returnvalue)
  (set `self.Blackboard` (`AIBlueprintHelperLibrary.GetBlackboard` self))
  (`KismetSystemLibrary.K2_SetTimerDelegate` (delegate `PostureRegen`) 2.0 true))

(event `PostureRegen`
  (bind _posture (`self.posture`))
  (if (<= _posture 5.0)
    (set `self.posture` (+ _posture 1.0))))

(event `self.ReceiveAnyDamage`
  (params (Damage :type "Float (single-precision)") (DamageType :type "DamageType Object Reference") (InstigatedBy :type "Controller Object Reference") (DamageCauser :type "Actor Object Reference"))
  (`self.Hit` Damage Damage)
  (`BlackboardComponent.SetValueAsEnum` (`AIBlueprintHelperLibrary.GetBlackboard` (`AIBlueprintHelperLibrary.GetAIController` self)) (`self.AIState`) 4)
  (`AISense_Damage.ReportDamageEvent` self DamageCauser Damage (`self.K2_GetActorLocation`))
  (`/Game/TH/Blueprints/BP_Manager.StartAI` (`self.AIManager`)))

(event `Dead`
  (`|PlayMontage` (`self.Mesh`) "/Game/TH/Animation/Mon_GuardBreakSet.Mon_GuardBreakSet" 1.0 0.0 "Death0"))

(event `PostureBreak`
  (`BlackboardComponent.SetValueAsBool` (`self.Blackboard`) (`self.Broken`) true))

(fn `Hit`
  (params (Damage :type "Float (double-precision)") (Posture :type "Float (double-precision)"))
  (bind _output_get (set `self.hp` (- (`self.hp`) Damage)))
  (bind _output_get_2 (set `self.posture` (- (`self.posture`) Posture)))
  (if (<= _output_get 0.0)
    (`self.Dead`)
    (else
      (if (<= _output_get_2 0.0)
        (`self.PostureBreak`))
      (return))))

(fn `UpdateMoveSpeed`
  (params (NewSpeed :type "Float (double-precision)"))
  (set `CharacterMovementComponent.MaxWalkSpeed` NewSpeed (`self.CharacterMovement`)))

(fn `UserConstructionScript`)