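; Animation notify that slices a body part off the player character's targeted Dummy at a chosen frame of an animation.
; It casts the mesh owner to PlayerCharacter and its EnemyTarget to Dummy, stopping if either cast fails.
; It calls SliceBodyPart on the dummy with the notify's body index, impulse and ragdoll delay, then turns off the player's targeting and clears the enemy target.
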(fn `Received_Notify`
  (params (MeshComp :type "SkeletalMeshComponent Object Reference") (Animation :type "AnimSequenceBase Object Reference") (EventReference :type "AnimNotifyEventReference Structure (by ref)"))
  (returns (ReturnValue :type Boolean))
  (bind _asplayer_character (cast `PlayerCharacter` (`ActorComponent.GetOwner` MeshComp)))
  (bind _asdummy (cast `Dummy` (`PlayerCharacter.EnemyTarget` _asplayer_character)))
  (`Dummy.SliceBodyPart` _asdummy (`self.Body Index`) (`self.Impulse`) (`self.Ragdoll Delay`))
  (set `PlayerCharacter.bIsTargeting` false _asplayer_character)
  (set `PlayerCharacter.EnemyTarget` null _asplayer_character) ; nullptr
  (return false))