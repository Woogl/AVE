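; Player character Blueprint layering takedowns, skill cinematics, ghost trails and HUD over a C++ base.
; MotionMorph motion-warps the takedown beside the enemy target, triggers its finisher reaction, then deals heavy delayed damage.
; Skill events share CameraMove, which blends to a sequence camera, plays the sequence and returns to the follow camera by timer.
; Possession creates stat, message and screen-cut widgets; EndGame shows game over, then reloads the level.
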(event `self.MotionMorph`
  (bind (_returnvalue_roll _returnvalue_pitch) (`KismetMathLibrary.BreakRotator` (`self.K2_GetActorRotation`)))
  (bind _returnvalue (`self.K2_GetActorLocation` (`self.EnemyTarget`)))
  (bind (_returnvalue_roll_2 _returnvalue_pitch_2 _returnvalue_yaw) (`KismetMathLibrary.BreakRotator` (`KismetMathLibrary.FindLookAtRotation` (`self.K2_GetActorLocation`) (`self.K2_GetActorLocation` (`self.EnemyTarget`)))))
  ;[1 1 1] 모션 워핑
  (`MotionWarpingComponent.AddOrUpdateWarpTargetFromLocationAndRotation` (`self.MotionWarpingComp`) "TakeDown01" (+ (* (`KismetMathLibrary.Normal` (- (`self.K2_GetActorLocation`) _returnvalue)) 80.0) _returnvalue) (`KismetMathLibrary.MakeRotator` _returnvalue_roll _returnvalue_pitch _returnvalue_yaw))
  (bind _asenemy_base (cast `EnemyBase` (`self.EnemyTarget`)))
  (bind _output_get (set `self.FinishedEnemy` _asenemy_base))
  (`EnemyBase.OnFinishered` _output_get)
  (`KismetSystemLibrary.Delay` 2.0)
  (`GameplayStatics.ApplyPointDamage` _output_get 5000.0 (`KismetMathLibrary.MakeVector` 0.0) (`GameplayStatics.MakeHitResult` false)))

(event `self.SpawnGhostTrail`
  ;[1 1 1] 잔상
  (`|SpawnActorFromClass` "/Game/Team/Woogle/BP_GhostTrail.BP_GhostTrail_C" (`SceneComponent.K2_GetComponentToWorld` (`self.Mesh`)) "AlwaysSpawn" "OverrideRootScale" null self null))

(event `/Game/Blueprints/BPI_Player.SetRInterpSpeed`
  (params (RInterpSpeed :type "Float (double-precision)"))
  ;[1 1 1] Anim Notify
  (set `self.RInterpSpeed` RInterpSpeed))

(event `self.ReceivePossessed`
  (params (NewController :type "Controller Object Reference"))
  ;[1 1 1] 체력/체간 위젯(임시), 0번 스킬 반갈죽 이펙트용 위젯
  (if (== (`self.GetController`) (`GameplayStatics.GetPlayerController` 0))
    (bind _returnvalue (`|CreateWidget` "/Game/Team/Mun/WBP_PlayerStat.WBP_PlayerStat_C"))
    (bind _output_get (set `self.Widget_PlayerStat` _returnvalue))
    (`UserWidget.AddToViewport` _output_get 0)
    (bind _returnvalue_2 (`|CreateWidget` "/Game/Team/Mun/JudgementCut/WBP_ScreenCut.WBP_ScreenCut_C"))
    (set `self.Widget_ScreenCut` _returnvalue_2)
    ;[1 1 1] 미션, 안내문
    (bind _returnvalue_3 (`|CreateWidget` "/Game/Team/Woogle/LevelDesign/WBP_Message.WBP_Message_C"))
    (bind _output_get_2 (set `self.Widget_Message` _returnvalue_3))
    (`UserWidget.AddToViewport` _output_get_2 0)))

(event `/Game/Blueprints/BPI_Player.ShowDirectiveMessage`
  (params (TextToShow :type Text))
  ;[1 1 1] 미션, 안내문
  (set `/Game/Team/Woogle/LevelDesign/WBP_Message.Directive` TextToShow (`self.Widget_Message`)))

(event `InputAction|ChangeSkill` :overrideparent false
  (params (Key :type "Key Structure"))
  (:`Pressed`
    (`/Game/Team/Mun/WBP_PlayerStat.ChangeSkill` (`self.Widget_PlayerStat`) (`self.CurSkill`))))

(event `self.PlayFinisherSequence`
  ;[1 1 1] 스킬 시퀀스
  (`self.CameraMove` (`self.Sequence_Finisher`)))

(event `InputAction|ChangeSpecialAttack` :overrideparent false
  (params (Key :type "Key Structure"))
  (:`Pressed`
    (`/Game/Team/Mun/WBP_PlayerStat.ChangeSpecialAttack` (`self.Widget_PlayerStat`) (`self.CurSpecialAttack`))))

(event `self.PlayLightningShockSequence`
  ;[1 1 1] 스킬 시퀀스
  (`self.CameraMove` (`self.Sequence_Lightning`)))

(event `/Game/Blueprints/BPI_Player.ShowMissionMessage`
  (params (TextToShow :type Text))
  ;[1 1 1] 미션, 안내문
  (set `/Game/Team/Woogle/LevelDesign/WBP_Message.Mission` TextToShow (`self.Widget_Message`)))

(event `self.PlayJudgementCutSequence`
  ;[1 1 1] 스킬 시퀀스
  (`self.CameraMove` (`self.Sequence_JudgementCut`)))

(event `InputAction|Skill` :overrideparent false
  (params (Key :type "Key Structure"))
  (:`Pressed`
    (`/Game/Team/Mun/WBP_PlayerStat.KatasiroChange` (`self.Widget_PlayerStat`) (`self.CurKatasiro`))))

(event `self.PlayEarthquakeSequence`
  ;[1 1 1] 스킬 시퀀스
  (`self.CameraMove` (`self.Sequence_Earthquake`)))

(event `self.EndGame`
  (bind _returnvalue (`|CreateWidget` "/Game/Team/Mun/WBP_GameOver.WBP_GameOver_C"))
  (`UserWidget.AddToViewport` _returnvalue 0)
  (`KismetSystemLibrary.Delay` 3.0)
  (bind _returnvalue_2 (`GameplayStatics.GetCurrentLevelName` true))
  (`GameplayStatics.OpenLevel` (`KismetStringLibrary.Conv_StringToName` _returnvalue_2)))

(fn `CameraMove`
  (params (Sequence :type "ActorSequenceComponent Object Reference"))
  (bind _sequenceplayer (`ActorSequenceComponent.SequencePlayer` Sequence))
  (`PlayerController.SetViewTargetWithBlend` (`GameplayStatics.GetPlayerController` 0) (`ChildActorComponent.ChildActor` (`self.SequenceCameraTarget`)) 0.2 "VTBlend_EaseInOut" 1.0 false)
  (`MovieSceneSequencePlayer.Play` _sequenceplayer)
  (`KismetSystemLibrary.K2_SetTimer` null "EndSequence" (`TimeManagementBlueprintLibrary.Conv_QualifiedFrameTimeToSeconds` (`MovieSceneSequencePlayer.GetDuration` _sequenceplayer))))

(fn `EndSequence`
  (`PlayerController.SetViewTargetWithBlend` (`GameplayStatics.GetPlayerController` 0) (`ChildActorComponent.ChildActor` (`self.FollowCameraTarget`)) 0.2 "VTBlend_EaseInOut" 1.0 false))

(fn `ScreenCut`
  (bind _widget_screencut (`self.Widget_ScreenCut`))
  (`/Game/Team/Mun/JudgementCut/WBP_ScreenCut.Init` _widget_screencut)
  (`UserWidget.AddToViewport` _widget_screencut 0))

(fn `UserConstructionScript`)